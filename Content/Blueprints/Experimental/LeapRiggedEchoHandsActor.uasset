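; Experimental Leap rigged hands actor with left and right hand meshes and two VR controller child actors.
; BeginPlay casts both child actors to VRController and assigns their hand side, while ShowHand toggles each mesh's visibility only when it changes.
; Reconstruct, run from the construction script, sets both meshes' collision from the EnablePhysicsCollision flag.
; The socket location and rotation getters query only the left hand mesh.
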(event `self.ReceiveBeginPlay`
  (`parent.ReceiveBeginPlay`)
  (bind _asvrcontroller (cast `/Game/Blueprints/Controller/VRController` (`ChildActorComponent.ChildActor` (`self.LController`))))
  (set `/Game/Blueprints/Controller/VRController.Hand` "Left" _asvrcontroller)
  (bind _asvrcontroller_2 (cast `/Game/Blueprints/Controller/VRController` (`ChildActorComponent.ChildActor` (`self.RController`))))
  (set `/Game/Blueprints/Controller/VRController.Hand` "Right" _asvrcontroller_2))

(event `self.ShowHand`
  (params (Hand :type "LeapHandType Enum" :default "HAND_UNKNOWN") (Visible :type Boolean))
  (bind _lefthandmesh (`self.LeftHandMesh`))
  (bind _righthandmesh (`self.RightHandMesh`))
  (switch `LeapHandType` Hand
    (:`HAND_LEFT`
      (if (!= (`SceneComponent.bVisible` _lefthandmesh) Visible)
        (`SceneComponent.SetVisibility` _lefthandmesh Visible false)))
    (:`HAND_RIGHT`
      (if (!= (`SceneComponent.bVisible` _righthandmesh) Visible)
        (`SceneComponent.SetVisibility` _righthandmesh Visible false)))))

(event `self.Reconstruct`
  (bind _lefthandmesh (`self.LeftHandMesh`))
  (if (`self.EnablePhysicsCollision`)
    (`PrimitiveComponent.SetCollisionEnabled` _lefthandmesh "QueryAndPhysics")
    (`PrimitiveComponent.SetCollisionEnabled` (`self.RightHandMesh`) "QueryAndPhysics")
    (else
      (`PrimitiveComponent.SetCollisionEnabled` _lefthandmesh "NoCollision")
      (`PrimitiveComponent.SetCollisionEnabled` (`self.RightHandMesh`) "NoCollision"))))

(fn `GetSocketLocation`
  (params (SocketName :type Name))
  (returns (Location :type "Vector Structure"))
  (return (`SceneComponent.GetSocketLocation` (`self.LeftHandMesh`) SocketName)))

(fn `GetSocketRotation`
  (params (Socket :type Name))
  (returns (Rotation :type "Rotator Structure"))
  (return (`SceneComponent.GetSocketRotation` (`self.LeftHandMesh`) Socket)))

(fn `UserConstructionScript`
  (`parent.UserConstructionScript`)
  (`self.Reconstruct`))