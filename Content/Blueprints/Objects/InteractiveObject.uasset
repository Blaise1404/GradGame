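; Interactive object actor with a tinted skeletal mesh and FMOD audio that can be brought to a target position and put away.
; A timeline lerps the mesh's location and scale toward the DATA actor's target and reverses on put-away; while active, Tick keeps it following that target with damping.
; Tick also samples amplitude and frequency arrays from a SoundWave at the FMOD playback position, for visualisation.
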(event `ChangeColor`
  (params (AddToHue :type "Float (double-precision)")))

(event `self.ReceiveBeginPlay`
  (set `self.MyScale` (`self.GetActorScale3D`))
  (bind _outactors (`GameplayStatics.GetAllActorsOfClass` "/Game/Blueprints/GameSettings/DATA.DATA_C"))
  (set `self.Data` (`KismetArrayLibrary.Array_Get` _outactors))
  (set `self.Start` (`SceneComponent.K2_GetComponentLocation` (`self.DefaultSceneRoot`))))

(event `bring`
  (bind _targetscale (`self.TargetScale`))
  (bind _mesh (`self.Mesh`))
  (set `self.Active` true)
  (bind (_direction _curve) (`Timeline|Move_timeline` :!label _label)
    (:`Update`
      (`SceneComponent.K2_SetWorldLocation` _mesh (`KismetMathLibrary.VLerp` (`self.Start`) (`/Game/Blueprints/GameSettings/DATA.TargetPosition` (`self.Data`)) _curve) false false)
      (`SceneComponent.SetWorldScale3D` _mesh (`KismetMathLibrary.VLerp` (`self.MyScale`) (`KismetMathLibrary.MakeVector` _targetscale _targetscale _targetscale) _curve)))))

(event `putAway`
  (set `self.Active` false)
  (goto _label :!via `Reverse`))

(event `self.ReceiveTick`
  (params (DeltaSeconds :type "Float (single-precision)"))
  (bind _mesh (`self.Mesh`))
  (`|ExecutionSequence`
    (:`then_0`
      (if (`self.Active`)
        (`SceneComponent.K2_SetWorldLocation` _mesh (`KismetMathLibrary.VLerp` (`SceneComponent.K2_GetComponentLocation` _mesh) (`/Game/Blueprints/GameSettings/DATA.TargetPosition` (`self.Data`)) (* DeltaSeconds (`self.Follow_dumping`))) false false)))
    (:`then_1`
      (`self.Visualiser`))))

(fn `ChangeHue`
  (params (Hue :type "Float (double-precision)") (Permanent :type Boolean))
  (if Permanent
    (bind (_h _s _v _a) (`KismetMathLibrary.RGBToHSV` (stale _output_get)))
    (bind _output_get (set `self.Color` (`KismetMathLibrary.HSVToRGB` (+ Hue _h) _s _v _a))))
  (`MaterialInstanceDynamic.SetVectorParameterValue` (`self.Material`) "Color" _output_get))

(fn `TimeElapsed`)

(fn `UserConstructionScript`
  (`|ExecutionSequence`
    (:`then_0`
      (`SkinnedMeshComponent.SetSkinnedAssetAndUpdate` (`self.Mesh`) (`self.MeshOverride`))
      (bind _returnvalue (`KismetMaterialLibrary.CreateDynamicMaterialInstance` (`self.BaseMaterial`)))
      (bind _output_get (set `self.Material` _returnvalue))
      (`PrimitiveComponent.SetMaterial` (`self.Mesh`) 0 _output_get)
      (`MaterialInstanceDynamic.SetVectorParameterValue` _output_get "Color" (`self.Color`)))
    (:`then_1`
      (`FMODAudioComponent.SetEvent` (`self.FMODAudio`) (`self.FModEvent`)))))

(fn `Visualiser`
  (bind _fmodaudio (`self.FMODAudio`))
  (bind _soundwave (`self.SoundWave`))
  (bind _returnvalue (`FMODAudioComponent.IsPlaying` _fmodaudio))
  (if _returnvalue
    (bind _returnvalue_2 (`FMODAudioComponent.GetTimelinePosition` _fmodaudio))
    (`|ExecutionSequence`
      (:`then_0`
        (bind _returnvalue_3 (/ (`KismetMathLibrary.Conv_IntToDouble` _returnvalue_2) 1000.0))
        (bind _outamplitudes (`SoundVisualizationStatics.GetAmplitude` _soundwave 0 _returnvalue_3 0.01 (`self.AmplitudeDivisions`)))
        (set `self.AmplitudeArray` _outamplitudes))
      (:`then_1`
        (bind _outspectrum (`SoundVisualizationStatics.CalculateFrequencySpectrum` _soundwave 0 _returnvalue_3 0.01 (`self.FrequencyDivisions`)))
        (set `self.FrequencyArray` _outspectrum)))))