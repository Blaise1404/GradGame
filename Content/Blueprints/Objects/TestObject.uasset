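; Test object that links a skeletal mesh's shape and color to an FMOD sound.
; ChangeShape nudges a clamped Shape value that drives both the anim instance's Time and the audio pitch.
; Tick normalizes the first amplitude value against its running peak and adds it to the animation as vibration, skipping new peaks while Active.
; Construction applies the hue, and BeginPlay maps the color's hue to an audio filter before starting playback.
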(event `self.ReceiveBeginPlay`
  (`parent.ReceiveBeginPlay`)
  (`self.UpdateFilter`)
  (`FMODAudioComponent.Play` (`self.FMODAudio`))
  (bind _asparent_anim (cast `/Game/Blueprints/ParentAnim` (`SkeletalMeshComponent.GetAnimInstance` (`self.Mesh`)) :!label _label))
  (set `/Game/Blueprints/ParentAnim.Time` (mod (+ (`self.Shape`) (`self.Vibration`)) (`self.max_shape`)) _asparent_anim)
  (`FMODAudioComponent.SetParameter` (`self.FMODAudio`) "Pitch -L" (/ (`self.Shape`) (`self.max_shape`))))

(event `ChangeShape`
  (params (Value :type "Float (double-precision)"))
  (bind _output_get (set `self.Shape` (`KismetMathLibrary.FClamp` (+ (stale _output_get) (/ Value 50.0)) 0.0 (`self.max_shape`))))
  (goto _label))

(event `self.ReceiveTick`
  (params (DeltaSeconds :type "Float (single-precision)"))
  (bind _item (`KismetArrayLibrary.Array_Get` (`self.AmplitudeArray`)))
  (`parent.ReceiveTick` DeltaSeconds)
  (if (> _item (`self.max`))
    (set `self.max` _item)
    (if (not (`self.Active`))
      (set `self.Vibration` (/ (/ _item (`self.max`)) 5.0) :!label _label_2)
      (goto _label))
    (else
      (goto _label_2))))

(fn `UpdateFilter`
  (`FMODAudioComponent.SetParameter` (`self.FMODAudio`) "Filter" (mod (/ (`KismetMathLibrary.RGBToHSV` (`self.Color`)) 360.0) 1.0)))

(fn `UserConstructionScript`
  (`parent.UserConstructionScript`)
  (`self.ChangeHue` (`self.Hue`) true))