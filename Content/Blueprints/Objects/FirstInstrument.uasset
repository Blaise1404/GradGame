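; FirstInstrument is a musical object whose HueTone sets both its construction-time color and the pitch of its FMOD audio.
; BeginPlay sets pitch and volume, and each Tick feeds the first AmplitudeArray value into a non-permanent hue change.
; The bring event runs a timeline that scales the mesh uniformly from the actor's X scale and starts the audio from a timeline event.
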(event `self.ReceiveBeginPlay`
  (bind _fmodaudio (`self.FMODAudio`))
  (`parent.ReceiveBeginPlay`)
  (`FMODAudioComponent.SetParameter` _fmodaudio "Pitch -S" (`self.Hue/Tone`))
  (`FMODAudioComponent.SetParameter` _fmodaudio "Volume" 0.5))

(event `self.ReceiveTick`
  (params (DeltaSeconds :type "Float (single-precision)"))
  (`parent.ReceiveTick` DeltaSeconds)
  (`self.ChangeHue` (`KismetArrayLibrary.Array_Get` (`self.AmplitudeArray`))))

(event `bring`
  (bind _output_get (set `self.Scale` (`self.GetActorScale3D`)))
  (bind (_direction _position) (`Timeline|MoveTimeline` :!via `PlayFromStart`)
    (:`Update`
      (bind _returnvalue (* (.x _output_get) _position))
      (`SceneComponent.SetWorldScale3D` (`self.Mesh`) (`KismetMathLibrary.MakeVector` _returnvalue _returnvalue _returnvalue)))
    (:`Event`
      (`FMODAudioComponent.Play` (`self.FMODAudio`)))))

(fn `UserConstructionScript`
  (`parent.UserConstructionScript`)
  (`self.ChangeHue` (* (`self.Hue/Tone`) 360.0) true))