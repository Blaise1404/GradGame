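; VR motion controller actor, one per hand, that lets the player beam, pull, edit and move the shared active InteractiveObject.
; A trigger-driven state machine (Play, Ray, Pull, Close, Edit, Move, Inactive) coordinates with the other controller and updates each tick.
; A line-traced spiral beam grabs objects; motion drives pull value, and wrist roll edits shape (left) or hue (right).
; State changes and overlaps drive per-hand sound and haptics.
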(event OnComponentBeginOverlap(Capsule)
  (params (OverlappedComponent :type Primitive%20Component%20Object%20Reference) (OtherActor :type Actor%20Object%20Reference) (OtherComp :type Primitive%20Component%20Object%20Reference) (OtherBodyIndex :type Integer) (bFromSweep :type Boolean) (SweepResult :type Hit%20Result%20Structure%20%28by%20ref%29))
  ;[1 1 1] Overlap events
)

(event OnComponentEndOverlap(Capsule)
  (params (OverlappedComponent :type Primitive%20Component%20Object%20Reference) (OtherActor :type Actor%20Object%20Reference) (OtherComp :type Primitive%20Component%20Object%20Reference) (OtherBodyIndex :type Integer))
  ;[1 1 1] Overlap events
)

(event OnComponentEndOverlap(collider)
  (params (OverlappedComponent :type Primitive%20Component%20Object%20Reference) (OtherActor :type Actor%20Object%20Reference) (OtherComp :type Primitive%20Component%20Object%20Reference) (OtherBodyIndex :type Integer))
  (bind _returnvalue (Game|GetPlayerController 0))
  ;[1 1 1] Overlap events
  (Utilities|Casting|CastToInteractiveObject OtherActor)
  (Class|FMODAudioComponent|Stop (Variables|Default|GetSoundEffects))
  (switch Utilities|FlowControl|Switch|SwitchonEControllerHand (Variables|Controller|GetHand)
    (:Left
      (Game|Feedback|ClientStopForceFeedback _returnvalue "/Game/Haptic/LIn.LIn" "L"))
    (:Right
      (Game|Feedback|ClientStopForceFeedback _returnvalue "/Game/Haptic/LIn.LIn" "R"))))

(event OnComponentBeginOverlap(collider)
  (params (OverlappedComponent :type Primitive%20Component%20Object%20Reference) (OtherActor :type Actor%20Object%20Reference) (OtherComp :type Primitive%20Component%20Object%20Reference) (OtherBodyIndex :type Integer) (bFromSweep :type Boolean) (SweepResult :type Hit%20Result%20Structure%20%28by%20ref%29))
  (bind _returnvalue (Game|GetPlayerController 0))
  (bind _hand (Variables|Controller|GetHand))
  (bind _soundeffects (Variables|Default|GetSoundEffects))
  ;[1 1 1] Overlap events
  (Utilities|Casting|CastToNoise OtherActor
    (:then
      (bind _returnvalue_2 (Physics|GetPhysicsLinearVelocity (Variables|Default|Getcollider) "None" :!label _label))
      (switch Utilities|FlowControl|Switch|SwitchonEControllerHand _hand
        (:Left
          (Game|Feedback|PlayDynamicForceFeedback _returnvalue (Math|Float|Clamp(Float) (/ (Math|Vector|VectorLength _returnvalue_2) 3e+02) 0.3) 0.1 true true false false))
        (:Right
          (Game|Feedback|PlayDynamicForceFeedback _returnvalue (Math|Float|Clamp(Float) (/ (Math|Vector|VectorLength _returnvalue_2) 3e+02) 0.3) 0.1 false false true true))))
    (:CastFailed
      (Utilities|Casting|CastToInstrument OtherActor
        (:then
          (goto _label))
        (:CastFailed
          (Utilities|Casting|CastToInteractiveObject OtherActor)
          (Class|FMODAudioComponent|SetParameter _soundeffects "0" 0.92)
          (Class|FMODAudioComponent|Play _soundeffects)
          (switch Utilities|FlowControl|Switch|SwitchonEControllerHand _hand
            (:Left
              (Game|Feedback|ClientPlayForceFeedback _returnvalue "/Game/Haptic/LIn.LIn" true "L"))
            (:Right
              (Game|Feedback|ClientPlayForceFeedback _returnvalue "/Game/Haptic/RIn.RIn" true "R"))))))))

(event Custom|Trigger%20Released
  (bind _soundeffects (Variables|Default|GetSoundEffects))
  (bind _soundeffects_2 (Variables|Default|GetSoundEffects))
  (bind _vrcharacter (Variables|Default|GetVRCharacter))
  ;[0.7049 1 0.687] Control v0.3
  ;;[0.4609 1 0.6363] Trigger
  (switch Utilities|FlowControl|Switch|SwitchonEControllerState (Variables|Controller|GetState)
    (:NewEnumerator12
      (CallFunction|StateChange "NewEnumerator0" :!label _label))
    (:NewEnumerator2
      (Variables|Pull|SetPullValue 0.0)
      (Class|FMODAudioComponent|SetParameter _soundeffects_2 "0" 0.82)
      (goto _label))
    (:NewEnumerator13
      (Class|FMODAudioComponent|SetParameter _soundeffects_2 "0" 0.72)
      (Class|FMODAudioComponent|Play _soundeffects_2))
    (:NewEnumerator11
      (CallFunction|StateChange "NewEnumerator13"))
    (:NewEnumerator4
      (if (> (- (.z (Transformation|GetWorldLocation (Variables|Default|GetMotionController))) (.z (.location (Variables|Default|GetTempTransform)))) 2e+01)
        (Default|MoveBelt _vrcharacter false)
        (CallFunction|StateChange "NewEnumerator0")
        (CallFunction|StateChange (Variables|Controller|GetOtherController) "NewEnumerator0")
        (Default|MoveDone (Variables|/Game/Blueprints/VR_Character.VR_Character_C|GetActiveObject _vrcharacter) true)
        (Variables|/Game/Blueprints/VR_Character.VR_Character_C|SetActiveObject (Variables|Default|GetVRCharacter) 0)
        (Class|FMODAudioComponent|SetParameter _soundeffects "0" 0.01)
        (Class|FMODAudioComponent|Play _soundeffects)
        (else
          (Default|MoveDone (Variables|/Game/Blueprints/VR_Character.VR_Character_C|GetActiveObject _vrcharacter) false)
          (CallFunction|StateChange "NewEnumerator13"))))))

(event Custom|Trigger%20Pressed
  (bind _othercontroller (Variables|Controller|GetOtherController))
  (bind _vrcharacter (Variables|Default|GetVRCharacter))
  (bind _activeobject (Variables|/Game/Blueprints/VR_Character.VR_Character_C|GetActiveObject _vrcharacter))
  ;[0.7049 1 0.687] Control v0.3
  ;;[0.4609 1 0.6363] Trigger
  (switch Utilities|FlowControl|Switch|SwitchonEControllerState (Variables|Controller|GetState)
    (:NewEnumerator0
      (bind _output_get (Variables|Pull|SetHue (Math|Random|RandomFloatinRange 0.0 1.0)))
      (Rendering|Material|SetScalarParameterValue (Variables|Default|GetMaterial) "Hue" _output_get :!class /Script/Engine.MaterialInstanceDynamic)
      (Components|Activation|Activate (Variables|Default|GetRay) true)
      (Rendering|Material|SetScalarParameterValue (Variables|Pull|GetBeamSpiralMat) "Hue" _output_get :!class /Script/Engine.MaterialInstanceDynamic)
      (Rendering|Material|SetScalarParameterValue (Variables|Pull|GetBeamMat) "Hue" _output_get :!class /Script/Engine.MaterialInstanceDynamic)
      (if (Utilities|IsValid (Variables|/Game/Blueprints/VR_Character.VR_Character_C|GetActiveObject (Variables|Default|GetVRCharacter)))
        (CallFunction|StateChange "NewEnumerator2")
        (else
          (CallFunction|StateChange "NewEnumerator12"))))
    (:NewEnumerator13
      (if (Collision|IsOverlappingActor (Variables|Default|Getcollider) _activeobject :!class /Script/Engine.PrimitiveComponent)
        (Transformation|SetWorldLocation (Variables|Default|GetMovePoint) (Transformation|GetWorldLocation (Variables|/Game/Blueprints/ObjectsBase/iObject.iObject_C|GetObject _activeobject)) false false)
        (Default|MoveStart _activeobject self)
        (CallFunction|StateChange "NewEnumerator4")
        (if (Utilities|Enum|Equal(Enum) (Variables|VRController_C|GetState _othercontroller) "NewEnumerator4")
          (CallFunction|StateChange _othercontroller "NewEnumerator13"))
        (else
          (CallFunction|StateChange "NewEnumerator11"))))))

(event EventBeginPlay
  (bind _ray (Variables|Default|GetRay))
  (bind _spiral (Variables|Default|GetSpiral))
  ;[1 1 1] Begin
  (Variables|Default|SetVRCharacter (.AsVR%20Character (Utilities|Casting|CastToVR_Character (Game|GetPlayerCharacter 0))))
  (bind _returnvalue (Rendering|Material|CreateDynamicMaterialInstance _spiral 0 (Rendering|Material|GetMaterial _spiral 0) :!class /Script/Engine.PrimitiveComponent))
  (Variables|Pull|SetBeamSpiralMat _returnvalue)
  (bind _returnvalue_2 (Rendering|Material|CreateDynamicMaterialInstance _ray 0 (Rendering|Material|GetMaterial _ray 0) :!class /Script/Engine.PrimitiveComponent))
  (Variables|Pull|SetBeamMat _returnvalue_2))

(event Collision|EventActorBeginOverlap
  (params (OtherActor :type Actor%20Object%20Reference)))

(event EventTick
  (params (DeltaSeconds :type Float%20%28single-precision%29))
  ;[1 1 1] Tick
  (CallFunction|StateBehaviour))

(fn ConstructionScript
  (bind _controller_mesh (Variables|Default|GetController%20Mesh))
  (bind _2side_arrow (Variables|Default|Get2side_arrow))
  (Utilities|FlowControl|Sequence
    (:then_0
      (bind _returnvalue (Rendering|Material|CreateDynamicMaterialInstance (Rendering|Material|GetMaterial _2side_arrow 0) :!class /Script/Engine.KismetMaterialLibrary))
      (Rendering|Material|SetMaterial _2side_arrow 0 _returnvalue))
    (:then_1
      (Variables|/Script/HeadMountedDisplay.MotionControllerComponent|SetHand (Variables|Default|GetMotionController) (Variables|Controller|GetHand))
      (bind _returnvalue_2 (Rendering|Material|CreateDynamicMaterialInstance (Rendering|Material|GetMaterial _controller_mesh 0) :!class /Script/Engine.KismetMaterialLibrary))
      (bind _output_get (Variables|Default|SetMaterial _returnvalue_2))
      (Rendering|Material|SetMaterial _controller_mesh 0 _output_get))))

(fn StateChange
  (params (To%20State :type EControllerState%20Enum))
  (bind _motioncontroller (Variables|Default|GetMotionController))
  (bind _beammat (Variables|Pull|GetBeamMat))
  (bind _ray (Variables|Default|GetRay))
  (bind _vrcharacter (Variables|Default|GetVRCharacter))
  (bind _spiral (Variables|Default|GetSpiral))
  (bind _vrcharacter_2 (Variables|Default|GetVRCharacter))
  (bind _returnvalue (Transformation|GetWorldTransform _motioncontroller))
  (bind _activeobject (Variables|/Game/Blueprints/VR_Character.VR_Character_C|GetActiveObject _vrcharacter))
  (bind _activeobject_2 (Variables|/Game/Blueprints/VR_Character.VR_Character_C|GetActiveObject _vrcharacter_2))
  ;[1 1 1] This function just changes state, update feedback, it is not validating
  (Utilities|FlowControl|Sequence
    (:then_0
      (if (!= To%20State (Variables|Controller|GetState))
        (switch Utilities|FlowControl|Switch|SwitchonEControllerState (Variables|Controller|GetState)
          (:NewEnumerator11
            ;;[1 1 1] Leave Action
            (Development|SetHiddeninGame (Variables|Default|Get2side_arrow) true false)))))
    (:then_1
      (bind _output_get (Variables|Controller|SetState To%20State))
      (switch Utilities|FlowControl|Switch|SwitchonEControllerState _output_get
        (:NewEnumerator0
          ;;[0.5372 1 0.376] Action
          ;;;[1 1 1] Play
          (if (Utilities|Enum|Equal(Enum) (Variables|VRController_C|GetState (Variables|Controller|GetOtherController)) "NewEnumerator2")
            _
            (else
              (Utilities|IsValid _activeobject
                (:Is%20Valid
                  (Default|PullEnd _activeobject))
                (:Is%20Not%20Valid
                  _))))
          ;;[1 0.968 0.3904] Controller Behaviour
          (Components|Activation|Deactivate _ray)
          (Development|SetHiddeninGame _spiral true false))
        (:NewEnumerator12
          ;;;[1 1 1] Ray
          (Development|SetHiddeninGame _spiral false false)
          (Effects|Components|ParticleSystem|SetVectorParameter (Variables|Default|GetRay) "SourceT" "0, 0, 0")
          (SplineMesh|SetEndScale _spiral "(X=4.000000,Y=4.000000)" false :!class /Script/Engine.SplineMeshComponent)
          (Rendering|Material|SetScalarParameterValue _beammat "Dir" 1.0 :!class /Script/Engine.MaterialInstanceDynamic)
          (Rendering|Material|SetScalarParameterValue _beammat "U" 1.0 :!class /Script/Engine.MaterialInstanceDynamic))
        (:NewEnumerator2
          ;;;[1 1 1] Pull
          (Variables|Default|SetTempTransform _returnvalue)
          (CallFunction|SetInitialDistance)
          (Default|PullStart (Variables|/Game/Blueprints/VR_Character.VR_Character_C|GetActiveObject (Variables|Default|GetVRCharacter)))
          (Development|SetHiddeninGame _spiral false false)
          (Rendering|Material|SetScalarParameterValue _beammat "Dir" -1.0 :!class /Script/Engine.MaterialInstanceDynamic)
          (Rendering|Material|SetScalarParameterValue _beammat "U" 2.0 :!class /Script/Engine.MaterialInstanceDynamic))
        (:NewEnumerator13
          ;;;[1 1 1] Close
          (Components|Activation|Deactivate _ray)
          (Development|SetHiddeninGame _spiral true false))
        (:NewEnumerator11
          ;;;[1 1 1] Edit
          (Variables|Default|SetTempTransform _returnvalue)
          (CallFunction|SetInitialDistance)
          (switch Utilities|FlowControl|Switch|SwitchonEControllerHand (Variables|Controller|GetHand)
            (:Left
              (Variables|Pull|SetBaseValue (Variables|/Game/Blueprints/ObjectsBase/InteractiveObject.InteractiveObject_C|GetShape _activeobject_2)))
            (:Right
              (Variables|Pull|SetBaseValue (Variables|/Game/Blueprints/ObjectsBase/iObject.iObject_C|GetHue _activeobject_2))))
          (Development|SetHiddeninGame (Variables|Default|Get2side_arrow) false false))
        (:NewEnumerator4
          _)
        (:NewEnumerator10
          ;;;[1 1 1] Inactive
          (Components|Activation|Deactivate _ray)
          (Development|SetHiddeninGame _spiral true false)))
      ;;[1 0.5997 0.04934] Sound
      (CallFunction|AudioHaptic))))

(fn StateBehaviour
  (bind _returnvalue (Utilities|Time|GetWorldDeltaSeconds))
  (bind _spiral (Variables|Default|GetSpiral))
  (bind _beamstart (Variables|Default|GetBeamStart))
  (bind _spiral_2 (Variables|Default|GetSpiral))
  (bind _ray (Variables|Default|GetRay))
  (bind _ray_2 (Variables|Default|GetRay))
  (bind _spiral_3 (Variables|Default|GetSpiral))
  (bind _beamstart_2 (Variables|Default|GetBeamStart))
  (bind _othercontroller (Variables|Controller|GetOtherController))
  (bind _motioncontroller (Variables|Default|GetMotionController))
  (bind _basevalue (Variables|Pull|GetBaseValue))
  (bind _returnvalue_2 (Transformation|GetWorldLocation _beamstart))
  (bind _returnvalue_3 (Math|Vector|GetForwardVector _motioncontroller))
  (bind _returnvalue_4 (Transformation|GetWorldLocation _beamstart_2))
  (bind _returnvalue_5 (* _returnvalue_3 9e+03))
  (switch Utilities|FlowControl|Switch|SwitchonEControllerState (Variables|Controller|GetState)
    (:NewEnumerator12
      ;[1 1 1] Ray
      (bind _output_get (Variables|Pull|SetRotation (+ (stale _output_get) (* (Utilities|Time|GetWorldDeltaSeconds) (LocalVariables|GetRotationSpeed)))))
      (Effects|Components|ParticleSystem|SetVectorParameter _ray "Source" _returnvalue_4)
      (Effects|Components|ParticleSystem|SetVectorParameter _ray "Target" _returnvalue_5)
      (Utilities|FlowControl|Sequence
        (:then_0
          (SplineMesh|SetStartandEnd _spiral _returnvalue_4 _returnvalue_3 _returnvalue_5 "0, 0,0.000000" false :!class /Script/Engine.SplineMeshComponent)
          (Class|SplineMeshComponent|SetStartRoll _spiral (Variables|Pull|GetRotation) false)
          (Class|SplineMeshComponent|SetEndRoll _spiral (+ (Variables|Pull|GetRotation) 8e+01) true))
        (:then_1
          (bind _outhit (Collision|LineTraceForObjects _returnvalue_4 _returnvalue_5 (Utilities|Array|MakeArray "ObjectTypeQuery4") false 0 "None"))
          (bind _asinteractive_object (Utilities|Casting|CastToInteractiveObject (.hitactor _outhit)))
          (Variables|/Game/Blueprints/VR_Character.VR_Character_C|SetActiveObject (Variables|Default|GetVRCharacter) _asinteractive_object)
          (CallFunction|StateChange "NewEnumerator2")
          (if (Utilities|Enum|Equal(Enum) (Variables|VRController_C|GetState _othercontroller) "NewEnumerator12")
            (CallFunction|StateChange _othercontroller "NewEnumerator2")))))
    (:NewEnumerator2
      ;[1 1 1] Pull
      (bind _output_get_2 (Variables|Pull|SetRotation (+ (stale _output_get_2) (* (Utilities|Time|GetWorldDeltaSeconds) (LocalVariables|GetRotationSpeed) -1.0))))
      (bind (_dist _roll _angle) (CallFunction|GetDistanceRotation))
      (Variables|Pull|SetPullValue (+ (/ _dist (LocalVariables|GetPullDistanceDivide)) (/ _angle (LocalVariables|GetPullRotationDivide))))
      (Utilities|FlowControl|Sequence
        (:then_0
          (SplineMesh|SetStartandEnd _spiral_2 _returnvalue_2 (* (Math|Interpolation|VInterpTo (/ (SplineMesh|GetStartTangent _spiral_3) 25) (* (Math|Vector|GetUpVector _beamstart) (+ (/ (Math|Vector|VectorLength (- (Transformation|GetWorldLocation (Variables|/Game/Blueprints/ObjectsBase/iObject.iObject_C|GetObject (Variables|/Game/Blueprints/VR_Character.VR_Character_C|GetActiveObject (Variables|Default|GetVRCharacter)))) _returnvalue_2)) 5e+01) 2.0)) _returnvalue 1e+01) 25.0) (Math|Interpolation|VInterpTo (SplineMesh|GetEndPosition _spiral_3) (Transformation|GetWorldLocation (Variables|/Game/Blueprints/ObjectsBase/iObject.iObject_C|GetObject (Variables|/Game/Blueprints/VR_Character.VR_Character_C|GetActiveObject (Variables|Default|GetVRCharacter)))) _returnvalue 1e+01) "0, 0, 0" false :!class /Script/Engine.SplineMeshComponent)
          (Class|SplineMeshComponent|SetStartRoll _spiral_2 (Variables|Pull|GetRotation) false)
          (Class|SplineMeshComponent|SetEndRoll _spiral_2 (+ (/ (Math|Vector|VectorLength (- (Transformation|GetWorldLocation (Variables|/Game/Blueprints/ObjectsBase/iObject.iObject_C|GetObject (Variables|/Game/Blueprints/VR_Character.VR_Character_C|GetActiveObject (Variables|Default|GetVRCharacter)))) _returnvalue_2)) 5e+01) (Variables|Pull|GetRotation) 1e+01) false)
          (SplineMesh|SetEndScale _spiral_2 (Math|Vector2D|MakeVector2D (+ (/ (Math|Vector|VectorLength (- (Transformation|GetWorldLocation (Variables|/Game/Blueprints/ObjectsBase/iObject.iObject_C|GetObject (Variables|/Game/Blueprints/VR_Character.VR_Character_C|GetActiveObject (Variables|Default|GetVRCharacter)))) _returnvalue_2)) 1.2e+03) 1.5) (+ (/ (Math|Vector|VectorLength (- (Transformation|GetWorldLocation (Variables|/Game/Blueprints/ObjectsBase/iObject.iObject_C|GetObject (Variables|/Game/Blueprints/VR_Character.VR_Character_C|GetActiveObject (Variables|Default|GetVRCharacter)))) _returnvalue_2)) 1.2e+03) 1.5)) true :!class /Script/Engine.SplineMeshComponent))
        (:then_1
          (Effects|Components|ParticleSystem|SetVectorParameter _ray_2 "Source" _returnvalue_2)
          (Effects|Components|ParticleSystem|SetVectorParameter _ray_2 "Target" (Math|Interpolation|VInterpTo (SplineMesh|GetEndPosition _spiral_3) (Transformation|GetWorldLocation (Variables|/Game/Blueprints/ObjectsBase/iObject.iObject_C|GetObject (Variables|/Game/Blueprints/VR_Character.VR_Character_C|GetActiveObject (Variables|Default|GetVRCharacter)))) _returnvalue 1e+01))
          (Effects|Components|ParticleSystem|SetVectorParameter _ray_2 "SourceT" (Math|Interpolation|VInterpTo (/ (SplineMesh|GetStartTangent _spiral_3) 25) (* (Math|Vector|GetUpVector _beamstart) (+ (/ (Math|Vector|VectorLength (- (Transformation|GetWorldLocation (Variables|/Game/Blueprints/ObjectsBase/iObject.iObject_C|GetObject (Variables|/Game/Blueprints/VR_Character.VR_Character_C|GetActiveObject (Variables|Default|GetVRCharacter)))) _returnvalue_2)) 5e+01) 2.0)) _returnvalue 1e+01)))))
    (:NewEnumerator11
      ;[1 1 1] Edit
      (bind _roll_2 (CallFunction|GetDistanceRotation))
      (switch Utilities|FlowControl|Switch|SwitchonEControllerHand (Variables|Controller|GetHand)
        (:Left
          (Default|ChangeShape (Variables|/Game/Blueprints/VR_Character.VR_Character_C|GetActiveObject (Variables|Default|GetVRCharacter)) _basevalue (/ _roll_2 (LocalVariables|GetEditRotationDivide))))
        (:Right
          (Default|ChangeHue (Variables|/Game/Blueprints/VR_Character.VR_Character_C|GetActiveObject (Variables|Default|GetVRCharacter)) _basevalue (/ _roll_2 (LocalVariables|GetEditRotationDivide))))))
    (:NewEnumerator4
      ;[1 1 1] Move
      (Transformation|SetRelativeRotation (Variables|/Game/Blueprints/ObjectsBase/iObject.iObject_C|GetObjectCentre (Variables|/Game/Blueprints/VR_Character.VR_Character_C|GetActiveObject (Variables|Default|GetVRCharacter))) (Math|Rotator|MakeRotator 0.0 0.0 (- (.yaw (Transformation|GetWorldRotation (Variables|Default|GetMotionController))) (+ (Variables|/Game/Blueprints/ObjectsBase/iObject.iObject_C|GetLocalYaw (Variables|/Game/Blueprints/VR_Character.VR_Character_C|GetActiveObject (Variables|Default|GetVRCharacter))) (Variables|/Game/Blueprints/ObjectsBase/iObject.iObject_C|GetGlobalYaw (Variables|/Game/Blueprints/VR_Character.VR_Character_C|GetActiveObject (Variables|Default|GetVRCharacter)))))) false false))))

(fn AudioHaptic
  (bind _returnvalue (Game|GetPlayerController 0))
  (bind _soundeffects (Variables|Default|GetSoundEffects))
  (bind _state (Variables|Controller|GetState))
  (switch Utilities|FlowControl|Switch|SwitchonEControllerHand (Variables|/Script/HeadMountedDisplay.MotionControllerComponent|GetHand (Variables|Default|GetMotionController))
    (:Left
      (switch Utilities|FlowControl|Switch|SwitchonEControllerState _state
        (:NewEnumerator0
          (Class|FMODAudioComponent|Stop _soundeffects :!label _label)
          (Game|Feedback|ClientStopForceFeedback _returnvalue 0 "L"))
        (:NewEnumerator12
          (Class|FMODAudioComponent|SetParameter _soundeffects "0" 0.12)
          (Game|Feedback|ClientPlayForceFeedback _returnvalue "/Game/Haptic/LBeam.LBeam" true "L")
          (Class|FMODAudioComponent|Play _soundeffects :!label _label_2))
        (:NewEnumerator2
          (Class|FMODAudioComponent|SetParameter _soundeffects "0" 0.62)
          (Game|Feedback|ClientPlayForceFeedback _returnvalue "/Game/Haptic/LPull.LPull" true "L")
          (goto _label_2))
        (:NewEnumerator13
          (goto _label))
        (:NewEnumerator4
          (Game|Feedback|ClientPlayForceFeedback _returnvalue "/Game/Haptic/LMove.LMove" true "L"))
        (:NewEnumerator10
          (goto _label))))
    (:Right
      (switch Utilities|FlowControl|Switch|SwitchonEControllerState _state
        (:NewEnumerator0
          (Class|FMODAudioComponent|Stop _soundeffects :!label _label_3)
          (Game|Feedback|ClientStopForceFeedback (Game|GetPlayerController 0) 0 "R"))
        (:NewEnumerator12
          (Class|FMODAudioComponent|SetParameter _soundeffects "0" 0.22)
          (Game|Feedback|ClientPlayForceFeedback _returnvalue "/Game/Haptic/RBeam.RBeam" true "R")
          (goto _label_2))
        (:NewEnumerator2
          (Class|FMODAudioComponent|SetParameter _soundeffects "0" 0.52)
          (Game|Feedback|ClientPlayForceFeedback _returnvalue "/Game/Haptic/RPull.RPull" true "R")
          (goto _label_2))
        (:NewEnumerator13
          (goto _label_3))
        (:NewEnumerator4
          (Game|Feedback|ClientPlayForceFeedback _returnvalue "/Game/Haptic/RMove.RMove" true "R"))
        (:NewEnumerator10
          (goto _label_3))))))

(fn SetControlValue
  (params (Rotation :type Boolean)))

(fn GetDistanceRotation
  (bind _temptransform (Variables|Default|GetTempTransform))
  (bind _motioncontroller (Variables|Default|GetMotionController))
  (bind _vrcharacter (Variables|Default|GetVRCharacter))
  (bind _returnvalue (Transformation|GetWorldRotation _motioncontroller))
  (bind _returnvalue_2 (Transformation|GetWorldLocation _motioncontroller))
  (bind _activeobject (Variables|/Game/Blueprints/VR_Character.VR_Character_C|GetActiveObject _vrcharacter))
  (bind _orbittarget (Variables|/Game/Blueprints/ObjectsBase/iObject.iObject_C|GetOrbitTarget _activeobject))
  (bind _returnvalue_3 (Transformation|GetWorldLocation _orbittarget))
  (return (- (Math|Vector|VectorLength (- (Math|Vector|MakeVector (.x _returnvalue_3) (.y _returnvalue_3) 0.0) (Math|Vector|MakeVector (.x _returnvalue_2) (.y _returnvalue_2) 0.0))) (Variables|Pull|GetStartDistance)) (.roll (Math|Rotator|Delta(Rotator) (.rotation _temptransform) _returnvalue)) (Class|KismetMathLibrary|DegAcos (Math|Vector|DotProduct (Math|Vector|Normalize (Math|Vector|GetForwardVector (.rotation _temptransform))) (Math|Vector|Normalize (Math|Vector|GetForwardVector _returnvalue))))))

(fn SetInitialDistance
  (bind _temptransform (Variables|Default|GetTempTransform))
  (bind _vrcharacter (Variables|Default|GetVRCharacter))
  (bind _activeobject (Variables|/Game/Blueprints/VR_Character.VR_Character_C|GetActiveObject _vrcharacter))
  (bind _orbittarget (Variables|/Game/Blueprints/ObjectsBase/iObject.iObject_C|GetOrbitTarget _activeobject))
  (bind _returnvalue (Transformation|GetWorldLocation _orbittarget))
  (Variables|Pull|SetStartDistance (Math|Vector|VectorLength (- (Math|Vector|MakeVector (.x (.location _temptransform)) (.y (.location _temptransform)) 0.0) (Math|Vector|MakeVector (.x _returnvalue) (.y _returnvalue) 0.0))))
  (return))