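; TestObject2 is a test actor whose mesh color and audio respond to player horizontal input.
; Construction creates a dynamic material with its Color, and BeginPlay applies the spikes, mid and out morph targets.
; PlayerHor shifts the hue and drives FMOD's "Drums?" parameter from it.
; PlayerVert ignores its input, freezing an animation at the Shape position, while morph-driven "Distance" audio logic sits disconnected.
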(event `self.ReceiveActorBeginOverlap`
  (params (OtherActor :type "Actor Object Reference")))

(event `self.ReceiveBeginPlay`
  (bind _mesh (`self.Mesh`))
  (`parent.ReceiveBeginPlay`)
  (`SkeletalMeshComponent.SetMorphTarget` _mesh "spikes" (`self.spikes`) true)
  (`SkeletalMeshComponent.SetMorphTarget` _mesh "mid" (`self.mid`) true)
  (`SkeletalMeshComponent.SetMorphTarget` _mesh "out" (`self.out`) true))

(event `Player Hor`
  (params (Value :type "Float (double-precision)"))
  (bind (_h _s _v _a) (`KismetMathLibrary.RGBToHSV` (stale _output_get)))
  (bind _returnvalue (+ Value _h))
  (bind _output_get (set `self.Color` (`KismetMathLibrary.HSVToRGB` _returnvalue _s _v _a)))
  (`MaterialInstanceDynamic.SetVectorParameterValue` (`self.Material`) "Color" (`self.Color`))
  (`FMODAudioComponent.SetParameter` (`self.FMODAudio`) "Drums?" (mod (/ _returnvalue 360.0) 1.0)))

(event `Player Vert`
  (params (Value :type "Float (double-precision)"))
  (set `SkeletalMeshComponent.AnimationData` (make `SingleAnimationPlayData` "/Game/Meshes/test/iso4anim_Anim.iso4anim_Anim" false false (`self.Shape`) 0.0) (`self.Mesh`)))

(fn `UserConstructionScript`
  (bind _returnvalue (`PrimitiveComponent.CreateDynamicMaterialInstance` (`self.Mesh`) 0 "/Game/Materials/TestMat.TestMat"))
  (set `self.Material` _returnvalue)
  (`MaterialInstanceDynamic.SetVectorParameterValue` (`self.Material`) "Color" (`self.Color`)))