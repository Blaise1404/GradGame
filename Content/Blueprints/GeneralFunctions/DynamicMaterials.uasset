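; DynamicMaterials is a set of general helper functions for creating dynamic materials and driving their visibility parameter.
; SetMaterials replaces every material slot on the given components with a dynamic instance of its current material and returns all the instances in one array.
; ApplyVis takes an array of such instances and sets their "Vis" scalar parameter to a given value.
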(fn `ApplyVis`
  (params (Materials :type "Array of MaterialInstanceDynamic Object Reference") (Vis :type "Float (double-precision)"))
  (for _array_element Materials
    (`MaterialInstanceDynamic.SetScalarParameterValue` _array_element "Vis" Vis)))

(fn `SetMaterials`
  (params (Objects :type "Array of MeshComponent Object Reference"))
  (returns (Materials :type "Array of MaterialInstanceDynamic Object Reference"))
  (locals (Mats :type "Array of MaterialInstanceDynamic Object Reference"))
  (bind _mats (`local.Mats`))
  (for _array_element Objects
    (for (_array_element_2 _array_index) (`MeshComponent.GetMaterials` _array_element)
      (bind _returnvalue (`KismetMaterialLibrary.CreateDynamicMaterialInstance` null _array_element_2))
      (`PrimitiveComponent.SetMaterial` _array_element _array_index _returnvalue)
      (`KismetArrayLibrary.Array_Add` _mats _returnvalue)))
  (return _mats))