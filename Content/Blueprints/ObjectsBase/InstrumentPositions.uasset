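; InstrumentPositions is an actor that provides a configurable number of position components around the VR player's instrument centre.
; The construction script keeps the first Amount of ten components, destroys the rest and pushes the survivors along their existing directions to a fixed radius, compensated for root scale.
; BeginPlay caches InstrumentCentre from VR_Character, and Tick interpolates the root's whole transform toward it at FollowSpeed for a smoothed follow.
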(event `self.ReceiveBeginPlay`
  (bind _asvr_character (cast `/Game/Blueprints/VR_Character` (`GameplayStatics.GetPlayerCharacter` 0)))
  (set `self.FollowCentre` (`/Game/Blueprints/VR_Character.InstrumentCentre` _asvr_character)))

(event `self.ReceiveTick`
  (params (DeltaSeconds :type "Float (single-precision)"))
  (`self.Follow`))

(fn `Follow`
  (bind _defaultsceneroot (`self.DefaultSceneRoot`))
  (`SceneComponent.K2_SetWorldTransform` _defaultsceneroot (`KismetMathLibrary.TInterpTo` (`SceneComponent.K2_GetComponentToWorld` _defaultsceneroot) (`SceneComponent.K2_GetComponentToWorld` (`self.FollowCentre`)) (`GameplayStatics.GetWorldDeltaSeconds`) (`self.FollowSpeed`)) false false))

(fn `UserConstructionScript`
  (bind _output_get (set `self.ArrayOfPositions` (`|MakeArray` (`self.0`) (`self.1`) (`self.2`) (`self.3`) (`self.4`) (`self.5`) (`self.6`) (`self.7`) (`self.8`) (`self.9`))))
  (for (_array_element _array_index) _output_get
    (if (not (< _array_index (`self.Amount`)))
      (`ActorComponent.K2_DestroyComponent` _array_element)))
  (`KismetArrayLibrary.Array_Resize` _output_get (`self.Amount`))
  (for _array_element_2 _output_get
    (`SceneComponent.K2_SetRelativeLocation` _array_element_2 (/ (* (`KismetMathLibrary.Normal` (`SceneComponent.RelativeLocation` _array_element_2)) 65.0) (`SceneComponent.RelativeScale3D` (`self.DefaultSceneRoot`))) false false)))