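; Instrument is an object that orbits a parent object and plays FMOD audio when a VR controller hits it, setting a parameter from hit velocity.
; While orbiting, it smoothly follows its centre and target and scales with the parent.
; FollowBelt, also bound to a debug F key, switches it to a belt slot chosen by ID, with a timeline driving follow speed and trail fade.
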(event `self.ReceiveBeginPlay`
  ;[1 1 1] Event Begin Play
  (`parent.ReceiveBeginPlay`)
  (bind _output_get (set `self.Centre` (`/Game/Blueprints/ObjectsBase/InteractiveObject.MyPos` (`self.ParentObject`))))
  (set `self.FollowSpeed` 10.0)
  (set `self.StartScale` (`SceneComponent.K2_GetComponentScale` _output_get)))

(event `Key|F` :consume false
  (params (Key :type "Key Structure" :default "AnyKey"))
  ;[1 0.01282 0] F Hack
  (:`Pressed`
    (`self.Follow Belt`)))

(event `self.ReceiveTick`
  (params (DeltaSeconds :type "Float (single-precision)"))
  (bind _centre (`self.Centre`))
  (bind _object (`self.Object`))
  (bind _currenttarget (`self.CurrentTarget`))
  ;[1 1 1] Event Tick
  (`|ExecutionSequence`
    (:`then_0`
      (switch `/Game/Blueprints/GeneralFunctions/EInstrumentTarget` (`self.State`)
        (:`NewEnumerator0`
          (`self.OrbitGlobal`)
          (`self.SmoothFollow` (`self.DefaultSceneRoot`) _centre)
          (`self.SetActorScale3D` (/ (`SceneComponent.K2_GetComponentScale` _centre) (`self.StartScale`)))
          (`self.SmoothFollow` _object _currenttarget))
        (:`NewEnumerator1`
          (`self.SmoothFollow` _object _currenttarget true true)))
      (`parent.ReceiveTick` (`GameplayStatics.GetWorldDeltaSeconds`)))))

(event `self.Collider.OnComponentBeginOverlap`
  (params (OverlappedComponent :type "PrimitiveComponent Object Reference") (OtherActor :type "Actor Object Reference") (OtherComp :type "PrimitiveComponent Object Reference") (OtherBodyIndex :type Integer) (bFromSweep :type Boolean) (SweepResult :type "HitResult Structure (by ref)"))
  (bind _asvrcontroller (cast `/Game/Blueprints/Controller/VRController` OtherActor))
  (bind _returnvalue (`PrimitiveComponent.GetPhysicsLinearVelocity` (`/Game/Blueprints/Controller/VRController.collider` _asvrcontroller) "None"))
  (`FMODAudioComponent.SetParameter` (`self.FMODAudio`) "0" (`KismetMathLibrary.FClamp` (/ (`KismetMathLibrary.VSize` _returnvalue) 200.0)))
  (`self.PlayFMod`))

(event `Follow Belt`
  (set `self.State` "NewEnumerator1")
  (bind _outactors (`GameplayStatics.GetAllActorsOfClass` "/Game/Blueprints/ObjectsBase/InstrumentPositions.InstrumentPositions_C"))
  (set `self.CurrentTarget` (`KismetArrayLibrary.Array_Get` (`/Game/Blueprints/ObjectsBase/InstrumentPositions.ArrayOfPositions` (`KismetArrayLibrary.Array_Get` _outactors)) (`self.ID`)))
  (bind (_direction _follow _opacity) (`Timeline|FollowSpeedControl`)
    (:`Update`
      (set `self.FollowSpeed` _follow)
      (`MaterialInstanceDynamic.SetScalarParameterValue` (`self.TrailMat`) "Opacity" _opacity))
    (:`Finished`
      (`ActorComponent.SetActive` (`self.Trail`) false false))))

(fn `FollowParrent`
  (`SceneComponent.K2_SetWorldLocation` (`self.DefaultSceneRoot`) (`SceneComponent.K2_GetComponentLocation` (`/Game/Blueprints/ObjectsBase/InteractiveObject.MyPos` (`self.ParentObject`))) false false))

(fn `StopFMod`
  (`FMODAudioComponent.Stop` (`self.FMODAudio`)))

(fn `UpdateScale`
  (`SceneComponent.SetWorldScale3D` (`self.Object`) (`KismetMathLibrary.Conv_DoubleToVector` (* (+ (`self.Amplitude`) 1.0) (`self.ObjectScaleFar`)))))

(fn `UserConstructionScript`
  (bind _output_get (set `self.Centre` (`/Game/Blueprints/ObjectsBase/InteractiveObject.MyPos` (`self.ParentObject`))))
  (`self.K2_SetActorLocation` (`SceneComponent.K2_GetComponentLocation` _output_get))
  (`parent.UserConstructionScript`))