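; Base actor for an orbiting satellite object that pairs a hue-shifting skeletal mesh with an FMOD event.
; Construction creates dynamic materials, assigns the event and places the mesh at its orbit target; Tick only spins the mesh.
; ChangeHue wraps hue into 0–1, feeding both materials and an FMOD parameter.
; Helpers not called here provide orbiting, interpolated following, playback and amplitude visualisation, sampling a SoundWave at the FMOD timeline position.
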(event `self.ReceiveBeginPlay`
  (`self.ChangeHue` (`self.Hue`)))

(event `self.ReceiveTick`
  (params (DeltaSeconds :type "Float (single-precision)"))
  (`self.OrbitLocal`))

(fn `AddKeep01`
  (params (Base :type "Float (double-precision)") (Add :type "Float (double-precision)"))
  (returns (Out :type "Float (double-precision)"))
  (bind _returnvalue (`KismetMathLibrary.Fraction` (+ Base Add)))
  (if (< _returnvalue 0.0)
    (return (+ _returnvalue 1.0))
    (else
      (return _returnvalue))))

(fn `ChangeHue`
  (params (Value :type "Float (double-precision)") (Add :type "Float (double-precision)"))
  (bind _output_get (set `self.Hue` (`self.AddKeep01` Value Add)))
  (`self.UpdateColors`)
  (`self.UpdateFmod` "0" _output_get)
  (return))

(fn `OrbitGlobal`
  (`SceneComponent.K2_AddLocalRotation` (`self.ObjectCentre`) (`KismetMathLibrary.MakeRotator` 0.0 0.0 (* (`self.OrbitSpeed`) (`GameplayStatics.GetWorldDeltaSeconds`))) false false)
  (return))

(fn `OrbitLocal`
  (`SceneComponent.K2_AddWorldRotation` (`self.Object`) (`KismetMathLibrary.MakeRotator` 0.0 0.0 (`self.SatelliteSpeed`)) false false))

(fn `PlayFMod`
  (`FMODAudioComponent.Play` (`self.FMODAudio`)))

(fn `SetOrbit`
  (bind _object (`self.Object`))
  (bind (_returnvalue_location _returnvalue_rotation _returnvalue_scale) (`KismetMathLibrary.BreakTransform` (`SceneComponent.K2_GetComponentToWorld` (`self.CurrentTarget`))))
  (`SceneComponent.K2_SetRelativeLocation` (`self.OrbitTarget`) (`KismetMathLibrary.MakeVector` (`self.Radius`)) false false)
  (`self.K2_SetActorRotation` (`KismetMathLibrary.MakeRotator` 0.0 (`self.Angle`) (`self.GlobalYaw`)))
  (`self.K2_AddActorLocalRotation` (`KismetMathLibrary.MakeRotator` 0.0 0.0 (`self.LocalYaw`)))
  (`SceneComponent.K2_SetRelativeRotation` (`self.Object`) (`KismetMathLibrary.MakeRotator` 0.0 (`self.SatelliteAngle`) (`self.SatelliteYaw`)) false false)
  (`SceneComponent.SetRelativeScale3D` (`self.OrbitTarget`) (`KismetMathLibrary.Conv_DoubleToVector` (`self.ObjectScaleFar`)))
  (set `self.CurrentTarget` (`self.OrbitTarget`))
  (`SceneComponent.SetWorldScale3D` (`self.OrbitPreview`) (`KismetMathLibrary.Conv_DoubleToVector` (`self.Radius`)))
  (`SceneComponent.K2_SetWorldTransform` _object (`KismetMathLibrary.MakeTransform` _returnvalue_location (`SceneComponent.K2_GetComponentRotation` _object) _returnvalue_scale) false false))

(fn `SmoothFollow`
  (params (Object :type "SceneComponent Object Reference") (Target :type "SceneComponent Object Reference") (Scale :type Boolean) (Rotation :type Boolean))
  (bind (_returnvalue_location _returnvalue_rotation _returnvalue_scale) (`KismetMathLibrary.BreakTransform` (`SceneComponent.K2_GetComponentToWorld` Object)))
  (bind _returnvalue (`GameplayStatics.GetWorldDeltaSeconds`))
  (bind _followspeed (`self.FollowSpeed`))
  (`SceneComponent.K2_SetWorldLocation` Object (`KismetMathLibrary.VInterpTo` _returnvalue_location (`SceneComponent.K2_GetComponentLocation` Target) _returnvalue _followspeed) false false)
  (if Scale
    (`SceneComponent.SetWorldScale3D` Object (`KismetMathLibrary.VInterpTo` _returnvalue_scale (`SceneComponent.RelativeScale3D` Target) _returnvalue _followspeed)))
  (if Rotation
    (`SceneComponent.K2_SetWorldRotation` Object (`KismetMathLibrary.RInterpTo` _returnvalue_rotation (`SceneComponent.K2_GetComponentRotation` Target) _returnvalue _followspeed) false false))
  (return))

(fn `UpdateColors`
  (for _array_element (`self.MaterialsDynamic`)
    (`MaterialInstanceDynamic.SetScalarParameterValue` _array_element "Hue" (+ (`self.InitialHue`) (`self.Hue`)))))

(fn `UpdateFmod`
  (params (Name :type Name) (Value :type "Float (double-precision)"))
  (returns (Result :type Boolean))
  (`FMODAudioComponent.SetParameter` (`self.FMODAudio`) Name (mod Value 1.0))
  (return true))

(fn `UserConstructionScript`
  (`|ExecutionSequence`
    (:`then_0`
      (`SkinnedMeshComponent.SetSkinnedAssetAndUpdate` (`self.Object`) (`self.Mesh`) true))
    (:`then_1`
      (for (_array_element _array_index) (`self.Materials`)
        (bind _returnvalue (`KismetMaterialLibrary.CreateDynamicMaterialInstance` _array_element))
        (`KismetArrayLibrary.Array_Set` (`self.MaterialsDynamic`) _array_index _returnvalue true)
        (`PrimitiveComponent.SetMaterial` (`self.Object`) _array_index _returnvalue)))
    (:`then_2`
      (`FMODAudioComponent.SetEvent` (`self.FMODAudio`) (`self.Fmod Event`)))
    (:`then_3`
      (`self.SetOrbit`)
      (`self.UpdateColors`))))

(fn `Visualiser`
  (bind _fmodaudio (`self.FMODAudio`))
  (bind _vis_wav_file (`self.Vis Wav File`))
  (bind _returnvalue (`FMODAudioComponent.IsPlaying` _fmodaudio))
  (if _returnvalue
    (`/Engine/EditorBlueprintResources/StandardMacros.IsValid` _vis_wav_file
      (:`Is Valid`
        (bind _returnvalue_2 (`FMODAudioComponent.GetTimelinePosition` _fmodaudio))
        (bind _outamplitudes (`SoundVisualizationStatics.GetAmplitude` _vis_wav_file 0 (+ (mod (/ (`KismetMathLibrary.Conv_IntToDouble` _returnvalue_2) 1000.0) (`SoundBase.Duration` _vis_wav_file)) (`self.Time Adjustment`)) (`self.Sample Lenght`) 1))
        (set `self.Amplitude` (`KismetMathLibrary.FClamp` (/ (`KismetArrayLibrary.Array_Get` _outamplitudes) (`self.AmplitudeDivide`)) 0.0 1.0))))))