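; A flying "Noise" object with a random hue and trail that sweeps past the VR player and bursts when touched by a VR controller.
; The root eases toward the player camera, carrying a long straight spline with random yaw; the mesh travels along it, offset to one side.
; Its speed scales with camera distance, slowing it near the player.
; A hit plays FMOD audio and physically scatters the mesh, then a timeline fades and shrinks it before destruction.
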(event `self.ReceiveBeginPlay`
  (bind _array (`|MakeArray` (10000.0 0.0 0.0) (-10000.0 0.0 0.0) :!type "Vector Structure"))
  (bind _z (`self.Z`))
  (`|ExecutionSequence`
    (:`then_0`
      (`KismetSystemLibrary.Delay` 1.0)
      (`ActorComponent.SetActive` (`self.Trail`) true true))
    (:`then_1`
      (`SplineComponent.SetSplinePoints` (`self.Spline`) _array "Local" true)
      (`SceneComponent.K2_SetWorldLocation` (`self.SkeletalMesh`) (`KismetArrayLibrary.Array_Get` _array 1) false true)
      (`self.K2_AddActorWorldRotation` (`KismetMathLibrary.MakeRotator` 0.0 0.0 (`KismetMathLibrary.RandomFloatInRange` 0.0 360.0)) false true)
      (if (`KismetMathLibrary.RandomBool`)
        (set `self.Offset` (`KismetMathLibrary.MakeVector` 0.0 65.0 _z))
        (else
          (set `self.Offset` (`KismetMathLibrary.MakeVector` 0.0 -65.0 _z)))))
    (:`then_2`
      (bind _output_get (set `self.Temp` (`KismetMathLibrary.RandomFloatInRange` 0.0 1.0)))
      (`MaterialInstanceDynamic.SetScalarParameterValue` (`self.TrailMat`) "Hue" _output_get)
      (for _array_element (`self.Materials Dynamic`)
        (`MaterialInstanceDynamic.SetScalarParameterValue` _array_element "Hue" _output_get)))))

(event `self.ReceiveTick`
  (params (DeltaSeconds :type "Float (single-precision)"))
  (bind _skeletalmesh (`self.SkeletalMesh`))
  ;[1 1 1] Tick
  (if (`self.Active`)
    (`self.SmoothFollow`)
    (bind _output_get (set `self.Position` (+ (stale _output_get) (/ (`KismetMathLibrary.VSize` (- (`SceneComponent.K2_GetComponentLocation` (`self.SkeletalMesh`)) (`SceneComponent.K2_GetComponentLocation` (`/Game/Blueprints/VR_Character.Camera` (`self.Character`))))) 100.0))))
    (if (> _output_get (`SplineComponent.GetSplineLength` (`self.Spline`)))
      (`self.K2_DestroyActor`)
      (else
        (`SceneComponent.K2_SetWorldLocation` _skeletalmesh (`SplineComponent.GetLocationAtDistanceAlongSpline` (`self.Spline`) _output_get "World") false true)
        (`SceneComponent.K2_AddLocalOffset` _skeletalmesh (`self.Offset`) false true)))))

(event `Destroyed`
  (bind _skeletalmesh (`self.SkeletalMesh`))
  (bind _fmodaudio (`self.FMODAudio`))
  (`FMODAudioComponent.SetParameter` _fmodaudio "0" 1.0 :!label _label)
  (`FMODAudioComponent.Play` _fmodaudio)
  (`PrimitiveComponent.SetCollisionEnabled` (`self.StaticMesh`) "NoCollision")
  (`ParticleSystemComponent.EndTrails` (`self.Trail`))
  (set `self.Active` false)
  (`PrimitiveComponent.SetSimulatePhysics` _skeletalmesh true)
  (`PrimitiveComponent.AddRadialForce` _skeletalmesh (- (`SceneComponent.K2_GetComponentLocation` _skeletalmesh) (* (`SceneComponent.GetUpVector` _skeletalmesh) -50.0)) 60.0 8000.0 "RIF_Constant" false)
  (set `self.Scale` (`SceneComponent.RelativeScale3D` (`self.SkeletalMesh`)))
  (bind (_direction _trail _pieces) (`Timeline|Timeline_0`)
    (:`Update`
      (`MaterialInstanceDynamic.SetScalarParameterValue` (`self.TrailMat`) "Opacity" _trail)
      (`SceneComponent.SetRelativeScale3D` (`self.SkeletalMesh`) (`KismetMathLibrary.VLerp` (0.0 0.0 0.0) (`self.Scale`) _pieces)))
    (:`Finished`
      (`self.K2_DestroyActor`))))

(event `self.StaticMesh.OnComponentBeginOverlap`
  (params (OverlappedComponent :type "PrimitiveComponent Object Reference") (OtherActor :type "Actor Object Reference") (OtherComp :type "PrimitiveComponent Object Reference") (OtherBodyIndex :type Integer) (bFromSweep :type Boolean) (SweepResult :type "HitResult Structure (by ref)"))
  (cast `/Game/Blueprints/Controller/VRController` OtherActor)
  (goto _label))

(fn `SmoothFollow`
  (bind _defaultsceneroot (`self.DefaultSceneRoot`))
  (`SceneComponent.K2_SetWorldLocation` _defaultsceneroot (`KismetMathLibrary.VInterpTo` (`SceneComponent.K2_GetComponentLocation` _defaultsceneroot) (`SceneComponent.K2_GetComponentLocation` (`/Game/Blueprints/VR_Character.Camera` (`self.Character`))) (`GameplayStatics.GetWorldDeltaSeconds`) (`self.FollowSpeed`)) false false))

(fn `UserConstructionScript`
  (bind _trail (`self.Trail`))
  (`|ExecutionSequence`
    (:`then_0`
      (bind _outactors (`GameplayStatics.GetAllActorsOfClass` "/Game/Blueprints/VR_Character.VR_Character_C"))
      (set `self.Character` (`KismetArrayLibrary.Array_Get` _outactors)))
    (:`then_1`
      (for (_array_element _array_index) (`self.Materials`)
        (bind _returnvalue (`KismetMaterialLibrary.CreateDynamicMaterialInstance` _array_element))
        (`KismetArrayLibrary.Array_Set` (`self.Materials Dynamic`) _array_index _returnvalue true)
        (`PrimitiveComponent.SetMaterial` (`self.SkeletalMesh`) _array_index _returnvalue)))
    (:`then_2`
      (bind _returnvalue_2 (`KismetMaterialLibrary.CreateDynamicMaterialInstance` (`PrimitiveComponent.GetMaterial` _trail 0)))
      (bind _output_get (set `self.TrailMat` _returnvalue_2))
      (`PrimitiveComponent.SetMaterial` _trail 0 _output_get))))