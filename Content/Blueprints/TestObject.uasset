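; TestObject is an actor that deforms its skeletal mesh by driving the Time variable of its iso4animBP animation blueprint.
; ChangeShape nudges a Shape value by scaled input, clamped to MaxShape.
; Tick derives a small Vibration offset from the first AmplitudeArray element, normalized against its running peak.
; BeginPlay, ChangeShape and Tick all write Shape plus Vibration, wrapped by MaxShape, into Time.
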(event `self.ReceiveActorBeginOverlap`
  (params (OtherActor :type "Actor Object Reference")))

(event `self.ReceiveBeginPlay`
  (`parent.ReceiveBeginPlay`)
  (bind _asiso_4anim_bp (cast `/Game/Meshes/test/iso4animBP` (`SkeletalMeshComponent.GetAnimInstance` (`self.Mesh`)) :!label _label))
  (set `/Game/Meshes/test/iso4animBP.Time` (mod (+ (`self.Shape`) (`self.Vibration`)) (`self.max_shape`)) _asiso_4anim_bp))

(event `ChangeShape`
  (params (Value :type "Float (double-precision)"))
  (bind _output_get (set `self.Shape` (`KismetMathLibrary.FClamp` (+ (stale _output_get) (/ Value 50.0)) 0.0 (`self.max_shape`))))
  (goto _label))

(event `self.ReceiveTick`
  (params (DeltaSeconds :type "Float (single-precision)"))
  (bind _item (`KismetArrayLibrary.Array_Get` (`self.AmplitudeArray`)))
  (`parent.ReceiveTick` DeltaSeconds)
  (if (> _item (`self.max`))
    (set `self.max` _item))
  (set `self.Vibration` (/ (/ _item (`self.max`)) 5.0))
  (goto _label))

(fn `UserConstructionScript`
  (`parent.UserConstructionScript`))