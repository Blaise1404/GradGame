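; VR interactive sound object that orbits the player and can be pulled close or held by a controller.
; An Orbit, Move, Close and Controller state machine switches the smooth-follow target and speed.
; While moving, both controllers' pull values drive a proxy target along a spline, and arrival moves the belt and releases child Instruments.
; A Shape value feeds an FMOD parameter and, offset by amplitude, animation time as a visualiser.
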(event Custom|MoveStart
  (params (Controller :type VR%20Controller%20Object%20Reference))
  ;[1 1 1] Move
  (CallFunction|UpdateState "NewEnumerator3" Controller))

(event Custom|MoveDone
  (params (Back :type Boolean))
  (bind _character (Variables|Default|GetCharacter))
  ;[1 1 1] Move
  (switch Utilities|FlowControl|Switch|SwitchonEObjectTarget (Variables|Basics|GetState)
    (:NewEnumerator6
      (if Back
        (CallFunction|UpdateState "NewEnumerator0")
        (else
          (Utilities|FlowControl|Sequence
            (:then_0
              (Default|MoveBelt _character true)
              (CallFunction|ReleaseInstruments))
            (:then_1
              (Default|StateChange (Variables|/Game/Blueprints/VR_Character.VR_Character_C|GetControllerR _character) "NewEnumerator13" :!label _label)
              (CallFunction|UpdateState "NewEnumerator2"))))))
    (:NewEnumerator3
      (if Back
        (CallFunction|UpdateState "NewEnumerator6")
        (Default|MoveBelt (Variables|Default|GetCharacter) false)
        (bind _value (Timeline|GoBack PlayFromStart)
          (:Update
            (Variables|PullPush|SetValue _value)))
        (else
          (goto _label))))))

(event Custom|PullEnd
  ;[1 1 1] Move
  (switch Utilities|FlowControl|Switch|SwitchonEObjectTarget (Variables|Basics|GetState)
    (:NewEnumerator6
      (CallFunction|UpdateState "NewEnumerator0")
      (Variables|/Game/Blueprints/VR_Character.VR_Character_C|SetActiveObject (Variables|Default|GetCharacter) 0))))

(event Custom|PullStart
  ;[1 1 1] Move
  (switch Utilities|FlowControl|Switch|SwitchonEObjectTarget (Variables|Basics|GetState)
    (:NewEnumerator0
      (CallFunction|UpdateState "NewEnumerator6")
      (Variables|PullPush|SetStartValue 0.1))
    (:NewEnumerator6
      (Variables|PullPush|SetDirBack false)
      (CallFunction|ResetTT)
      (Variables|PullPush|SetStartValue (Variables|PullPush|GetValue))
      (bind _value (Timeline|GoBack Stop)
        (:Update
          (Variables|PullPush|SetValue _value))))))

(event EventBeginPlay
  ;[1 1 1] Begin Play
  (Utilities|FlowControl|Sequence
    (:then_0
      (CallFunction|UpdateShape 0.0)
      (|CallParentFunction)
      (CallFunction|UpdateState "NewEnumerator0")
      (CallFunction|ChangeShape (Variables|Setup|GetShape) 0.0)
      (Transformation|SetWorldTransform (Variables|Default|GetTempTarget) (Transformation|GetWorldTransform (Variables|Default|GetOrbitTarget)) false false))))

(event EventActorBeginOverlap
  (params (OtherActor :type Actor%20Object%20Reference)))

(event EventTick
  (params (DeltaSeconds :type Float%20%28single-precision%29))
  (bind _currenttarget (Variables|Default|GetCurrentTarget))
  ;[1 1 1] EventTick
  (Utilities|FlowControl|Sequence
    (:then_0
      ;[1 1 1] Orbit
      (CallFunction|OrbitGlobal)
      (|CallParentFunction DeltaSeconds)
      (Utilities|IsValid _currenttarget
        (:Is%20Valid
          (CallFunction|SmoothFollow (Variables|Default|GetObject) _currenttarget true (Variables|Default|GetFollowRot)))))
    (:then_1
      ;[1 1 1] Visualiser
      (CallFunction|Visualiser)
      (CallFunction|UpdateShape (Variables|Default|GetAmplitude)))
    (:then_2
      ;[1 1 1] State behaviour
      (switch Utilities|FlowControl|Switch|SwitchonEObjectTarget (Variables|Basics|GetState)
        (:NewEnumerator0
          (CallFunction|SmoothFollow (Variables|Default|GetTempTarget) (Variables|Default|GetOrbitTarget) true false))
        (:NewEnumerator6
          (CallFunction|UpdatePull))))))

(fn ConstructionScript
  (bind _outactors (Actor|GetAllActorsOfClass "/Game/Blueprints/VR_Character.VR_Character_C"))
  (bind _output_get (Variables|Default|SetCharacter (Utilities|Array|Get(acopy) _outactors)))
  (Variables|Default|SetCentre (Variables|/Game/Blueprints/VR_Character.VR_Character_C|GetMainOrbitCentre _output_get))
  (|CallParentFunction)
  (Transformation|AddActorWorldOffset (Math|Vector|MakeVector 0.0 0.0 (Variables|Setup|GetCentreZOffset))))

(fn ChangeShape
  (params (Value :type Float%20%28single-precision%29) (Add :type Float%20%28single-precision%29))
  (bind _output_get (Variables|Setup|SetShape (CallFunction|AddKeep01 Value Add)))
  (CallFunction|UpdateFmod "1" _output_get)
  (CallFunction|UpdateShape 0.0))

(fn UpdateShape
  (params (AdditionalValue :type Float%20%28single-precision%29))
  (bind _asanim_interface (Utilities|Casting|CastToAnimInterface (Components|SkeletalMesh|GetAnimInstance (Variables|Default|GetObject))))
  (Default|ChangeTime _asanim_interface (CallFunction|AddKeep01 (Variables|Setup|GetShape) AdditionalValue)))

(fn UpdateState
  (params (State :type EObjectTarget%20Enum) (Controller :type VR%20Controller%20Object%20Reference))
  (bind _temptarget (Variables|Default|GetTempTarget))
  (switch Utilities|FlowControl|Switch|SwitchonEObjectTarget State
    (:NewEnumerator0
      ;[1 1 1] Action
      (Variables|PullPush|SetDirBack false)
      ;[1 1 1] Target
      (Variables|Default|SetCurrentTarget _temptarget)
      ;[1 1 1] Follow Speed
      (Variables|Default|SetFollowSpeed 1.5))
    (:NewEnumerator6
      (CallFunction|ResetTT)
      (Variables|Default|SetCurrentTarget _temptarget)
      (Variables|Default|SetFollowSpeed 4.0))
    (:NewEnumerator2
      (Variables|PullPush|SetDirBack true)
      (Variables|Default|SetCurrentTarget (Variables|/Game/Blueprints/VR_Character.VR_Character_C|GetCloseTarget (Variables|Default|GetCharacter)))
      (Variables|Default|SetFollowSpeed 2.0))
    (:NewEnumerator3
      (Variables|Default|SetCurrentTarget (Variables|/Game/Blueprints/VRController.VRController_C|GetMovePoint Controller))
      (Variables|Default|SetFollowSpeed 15.0)))
  (Variables|Basics|SetState State))

(fn UpdatePull
  (bind _pullspline (Variables|Default|GetPullSpline))
  (bind _temptarget (Variables|Default|GetTempTarget))
  (bind _value (Variables|PullPush|GetValue))
  (bind _character (Variables|Default|GetCharacter))
  (bind _object (Variables|Default|GetObject))
  (bind _orbittarget (Variables|Default|GetOrbitTarget))
  (bind _returnvalue (Transformation|GetWorldLocation _object))
  (bind _returnvalue_2 (Transformation|GetWorldLocation _orbittarget))
  (bind _returnvalue_3 (Transformation|GetWorldScale _orbittarget))
  (bind _closetarget (Variables|/Game/Blueprints/VR_Character.VR_Character_C|GetCloseTarget _character))
  (bind _returnvalue_4 (Transformation|GetWorldLocation _closetarget))
  (if (Variables|PullPush|GetDirBack)
    _
    (else
      (CallFunction|CalculateMoveValue)))
  (CallFunction|SetSpline _returnvalue_2 _returnvalue_4 "0, 0,0.000000" (Variables|PullPush|GetPullTangent))
  (if (Variables|PullPush|GetDirBack)
    (if (< (Math|Vector|VectorLength (- _returnvalue_2 _returnvalue)) 1e+02)
      (CallFunction|MoveDone true)
      (else
        (Transformation|SetWorldScale3D _temptarget (Math|Vector|Lerp(Vector) _returnvalue_3 (Transformation|GetWorldScale (Variables|/Game/Blueprints/VRController.VRController_C|GetMovePoint (Variables|/Game/Blueprints/VR_Character.VR_Character_C|GetControllerL _character))) _value))
        (Transformation|SetWorldLocation _temptarget (Spline|GetLocationatDistanceAlongSpline _pullspline (* (Spline|GetSplineLength _pullspline) _value) "World") false false :!label _label)))
    (elif (< (Math|Vector|VectorLength (- _returnvalue_4 _returnvalue)) 1e+02)
      (CallFunction|MoveDone false)
      (else
        (Transformation|SetWorldScale3D _temptarget (Math|Vector|Lerp(Vector) _returnvalue_3 (Transformation|GetWorldScale _closetarget) _value))
        (goto _label)))))

(fn ReleaseInstruments
  (bind _outactors (Actor|GetAllActorsOfClass "/Game/Blueprints/Object/Instrument.Instrument_C"))
  (for _array_element _outactors
    (if (== (Variables|/Game/Blueprints/Object/Instrument.Instrument_C|GetParentObject _array_element) self)
      (Default|FollowBelt _array_element))))

(fn Activation
  (params (Active :type Boolean))
  (bind _capsule (Variables|Default|GetCapsule))
  (bind _fmodaudio (Variables|Default|GetFMODAudio))
  (bind _output_get (Variables|Default|SetActive Active))
  (if _output_get
    (Collision|SetCollisionObjectType _capsule "ECC_PhysicsBody")
    (Class|FMODAudioComponent|Play _fmodaudio)
    (else
      (Collision|SetCollisionObjectType _capsule "ECC_Destructible")
      (Class|FMODAudioComponent|Stop _fmodaudio))))

(fn SetSpline
  (params (Start :type Vector) (End :type Vector) (StartTangent :type Vector) (EndTangent :type Vector))
  (bind _pullspline (Variables|Default|GetPullSpline))
  (Spline|SetLocationatSplinePoint _pullspline 0 Start "World")
  (Spline|SetLocationatSplinePoint _pullspline 1 End "World")
  (Spline|SetTangentatSplinePoint _pullspline 0 StartTangent "World")
  (Spline|SetTangentatSplinePoint _pullspline 1 EndTangent "World"))

(fn CalculateMoveValue
  (bind _character (Variables|Default|GetCharacter))
  (bind _startvalue (Variables|PullPush|GetStartValue))
  (bind _controllerl (Variables|/Game/Blueprints/VR_Character.VR_Character_C|GetControllerL _character))
  (bind _controllerr (Variables|/Game/Blueprints/VR_Character.VR_Character_C|GetControllerR _character))
  (bind _pullvalue (Variables|/Game/Blueprints/VRController.VRController_C|GetPullValue _controllerr))
  (bind _pullvalue_2 (Variables|/Game/Blueprints/VRController.VRController_C|GetPullValue _controllerl))
  (bind _output_get (Variables|PullPush|SetValue (Math|Interpolation|FInterpTo (stale _output_get) (+ _startvalue (* (- 1.0 _startvalue) (Math|Float|Clamp(Float) (+ (Math|Float|Max(Float) _pullvalue _pullvalue_2) (* (Math|Float|Min(Float) _pullvalue _pullvalue_2) 0.5))))) (Utilities|Time|GetWorldDeltaSeconds) (Variables|Default|GetFollowSpeed)))))

(fn ResetTT
  (bind _object (Variables|Default|GetObject))
  (bind _returnvalue (Transformation|GetWorldTransform _object))
  (Transformation|SetWorldTransform (Variables|Default|GetTempTarget) (Math|Transform|MakeTransform (.location _returnvalue) "0, 0, 0" (.scale _returnvalue)) false false))