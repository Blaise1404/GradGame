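; Instrument is a VR musical object that orbits a parent object or sits in a belt slot, playing FMOD audio when the VR character touches it.
; A state drives Tick: Orbit adds global orbit and parent following, while both states spin locally and smooth-follow the current target.
; Pressing F moves it to the belt position matching its ID.
; While audio plays, a visualiser runs and mesh scale follows amplitude.
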(event `self.ReceiveBeginPlay`
  (`parent.ReceiveBeginPlay`))

(event `Key|F` :consume false
  (params (Key :type "Key Structure" :default "AnyKey"))
  (:`Pressed`
    (`self.FollowBelt`)))

(event `self.ReceiveTick`
  (params (DeltaSeconds :type "Float (single-precision)"))
  (`|ExecutionSequence`
    (:`then_0`
      (switch `/Game/Blueprints/Object/EInstrumentTarget` (`self.State`)
        (:`NewEnumerator0`
          (`self.OrbitateGlobal`)
          (`self.OrbitateLocal`)
          (`self.FollowParrent`)
          (`self.SmoothFollow` DeltaSeconds))
        (:`NewEnumerator1`
          (`self.OrbitateLocal`)
          (`self.SmoothFollow` DeltaSeconds))))
    (:`then_1`
      (bind _returnvalue (`FMODAudioComponent.IsPlaying` (`self.FMODAudio`)))
      (if _returnvalue
        (`self.Visualiser`)
        (`self.UpdateScale`)))))

(event `self.SkeletalMesh.OnComponentBeginOverlap`
  (params (OtherActor :type "Actor Object Reference") (OtherComp :type "PrimitiveComponent Object Reference") (OtherBodyIndex :type Integer) (bFromSweep :type Boolean) (SweepResult :type "HitResult Structure (by ref)"))
  (if (`|EnumEquality` (`self.State`) "NewEnumerator1")
    (cast `/Game/Blueprints/VR_Character` OtherActor)
    (`self.PlayFMod`)))

(fn `FollowBelt`
  (set `self.State` "NewEnumerator1")
  (bind _outactors (`GameplayStatics.GetAllActorsOfClass` "/Game/Blueprints/Object/InstrumentPositions.InstrumentPositions_C"))
  (set `self.CurrentTarget` (`KismetArrayLibrary.Array_Get` (`/Game/Blueprints/Object/InstrumentPositions.ArrayOfPositions` (`KismetArrayLibrary.Array_Get` _outactors)) (`self.ID`))))

(fn `FollowObject`
  (set `self.State` "NewEnumerator0")
  (set `self.CurrentTarget` (`self.OrbitTarget`)))

(fn `FollowParrent`
  (`SceneComponent.K2_SetWorldLocation` (`self.DefaultSceneRoot`) (`SceneComponent.K2_GetComponentLocation` (`/Game/Blueprints/Object/InteractiveObject.MyPos` (`self.ParentObject`))) false false))

(fn `UpdateScale`
  (`SceneComponent.SetWorldScale3D` (`self.SkeletalMesh`) (`KismetMathLibrary.Conv_DoubleToVector` (* (+ (`self.Amplitude`) 1.0) (`self.ObjectScaleFar`)))))

(fn `UpdateState`
  (params (State :type "/Game/Blueprints/Object/EInstrumentTarget Enum"))
  (switch `/Game/Blueprints/Object/EInstrumentTarget` State
    (:`NewEnumerator0`
      (set `self.CurrentTarget` (`self.OrbitTarget`))
      (set `self.Centre` (`/Game/Blueprints/Object/InteractiveObject.MyPos` (`self.ParentObject`))))))

(fn `UserConstructionScript`
  (set `self.Centre` (`/Game/Blueprints/Object/InteractiveObject.MyPos` (`self.ParentObject`)))
  (`parent.UserConstructionScript`))