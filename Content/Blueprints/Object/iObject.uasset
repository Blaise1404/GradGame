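; Base object actor: a skeletal mesh that orbits a centre point, with a shared Hue driving both its materials and its FMOD audio.
; Construction applies the mesh, dynamic materials and FMOD event, then places the mesh from orbit settings; Tick rotates ObjectCentre.
; ChangeHue updates material and FMOD parameters together.
; Helpers, uncalled here, provide smooth following and derive amplitude from a sound wave synced to the FMOD timeline.
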(event `self.ReceiveBeginPlay`
  (`self.ChangeHue` (`self.Hue`)))

(event `self.ReceiveTick`
  (params (DeltaSeconds :type "Float (single-precision)"))
  (`self.OrbitLocal` false))

(fn `AddKeep01`
  (params (Base :type "Float (double-precision)") (Add :type "Float (double-precision)"))
  (returns (Out :type "Float (double-precision)"))
  (bind _returnvalue (`KismetMathLibrary.Fraction` (+ Base Add)))
  (if (< _returnvalue 0.0)
    (return (+ _returnvalue 1.0))
    (else
      (return _returnvalue))))

(fn `ChangeHue`
  (params (Value :type "Float (double-precision)"))
  (bind _output_get (set `self.Hue` Value))
  (`self.UpdateColors`)
  (`self.UpdateFmod` "0" _output_get))

(fn `OrbitGlobal`
  (`SceneComponent.K2_AddLocalRotation` (`self.SkeletalMesh`) (`KismetMathLibrary.MakeRotator` 0.0 0.0 (`self.SatelliteSpeed`)) false false))

(fn `OrbitLocal`
  (params (NewParam :type Boolean))
  (`SceneComponent.K2_AddLocalRotation` (`self.ObjectCentre`) (`KismetMathLibrary.MakeRotator` 0.0 0.0 (* (`self.OrbitSpeed`) (`GameplayStatics.GetWorldDeltaSeconds`))) false false))

(fn `PlayFMod`
  (bind _returnvalue (`FMODAudioComponent.IsPlaying` (`self.FMODAudio`)))
  (if (not _returnvalue)
    (`FMODAudioComponent.Play` (`self.FMODAudio`))))

(fn `SetOrbit`
  (bind _skeletalmesh (`self.SkeletalMesh`))
  (bind (_returnvalue_location _returnvalue_rotation _returnvalue_scale) (`KismetMathLibrary.BreakTransform` (`SceneComponent.K2_GetComponentToWorld` (`self.CurrentTarget`))))
  (`SceneComponent.K2_SetRelativeLocation` (`self.OrbitTarget`) (`KismetMathLibrary.MakeVector` (`self.OrbitRadius`)) false false)
  (`self.K2_SetActorRelativeTransform` (`KismetMathLibrary.MakeTransform` (`SceneComponent.K2_GetComponentLocation` (`self.Centre`)) (`KismetMathLibrary.MakeRotator` 0.0 (`self.OrbitAngle`) (`self.OrbitDir`))) false true)
  (`SceneComponent.K2_SetRelativeRotation` (`self.SkeletalMesh`) (`KismetMathLibrary.MakeRotator` 0.0 (`self.SatelliteAngle`)) false false)
  (`SceneComponent.SetRelativeScale3D` (`self.OrbitTarget`) (`KismetMathLibrary.Conv_DoubleToVector` (`self.ObjectScaleFar`)))
  (set `self.CurrentTarget` (`self.OrbitTarget`))
  (`SceneComponent.SetWorldScale3D` (`self.OrbitPreview`) (`KismetMathLibrary.Conv_DoubleToVector` (`self.OrbitRadius`)))
  (`SceneComponent.K2_SetWorldTransform` _skeletalmesh (`KismetMathLibrary.MakeTransform` _returnvalue_location (`SceneComponent.K2_GetComponentRotation` _skeletalmesh) _returnvalue_scale) false false))

(fn `SmoothFollow`
  (params (Object :type "SceneComponent Object Reference") (Target :type "SceneComponent Object Reference") (`With Scale` :type Boolean))
  (bind (_returnvalue_location _returnvalue_rotation _returnvalue_scale) (`KismetMathLibrary.BreakTransform` (`SceneComponent.K2_GetComponentToWorld` Target)))
  (bind (_returnvalue_location_2 _returnvalue_rotation_2 _returnvalue_scale_2) (`KismetMathLibrary.BreakTransform` (`SceneComponent.K2_GetComponentToWorld` Object)))
  (bind _returnvalue (`GameplayStatics.GetWorldDeltaSeconds`))
  (bind _followspeed (`self.FollowSpeed`))
  (`SceneComponent.K2_SetWorldLocation` Object (`KismetMathLibrary.VInterpTo` _returnvalue_location_2 _returnvalue_location _returnvalue _followspeed) false false)
  (if `With Scale`
    (`SceneComponent.SetWorldScale3D` Object (`KismetMathLibrary.VInterpTo` _returnvalue_scale_2 _returnvalue_scale _returnvalue _followspeed))))

(fn `UpdateColors`
  (for _array_element (`self.MaterialsDynamic`)
    (`MaterialInstanceDynamic.SetScalarParameterValue` _array_element "Hue" (`self.Hue`))))

(fn `UpdateFmod`
  (params (Name :type Name) (Value :type "Float (double-precision)"))
  (returns (Result :type Boolean))
  (`FMODAudioComponent.SetParameter` (`self.FMODAudio`) Name (mod Value 1.0))
  (return true))

(fn `UserConstructionScript`
  (`|ExecutionSequence`
    (:`then_0`
      (`SkinnedMeshComponent.SetSkinnedAssetAndUpdate` (`self.SkeletalMesh`) (`self.Mesh`) true))
    (:`then_1`
      (for (_array_element _array_index) (`self.Materials`)
        (bind _returnvalue (`KismetMaterialLibrary.CreateDynamicMaterialInstance` _array_element))
        (`KismetArrayLibrary.Array_Set` (`self.MaterialsDynamic`) _array_index _returnvalue true)
        (`PrimitiveComponent.SetMaterial` (`self.SkeletalMesh`) _array_index _returnvalue)))
    (:`then_2`
      (`FMODAudioComponent.SetEvent` (`self.FMODAudio`) (`self.Fmod Event`)))
    (:`then_3`
      (`self.SetOrbit`)
      (`self.UpdateColors`))))

(fn `Visualiser`
  (bind _fmodaudio (`self.FMODAudio`))
  (bind _vis_wav_file (`self.Vis Wav File`))
  (bind _returnvalue (`FMODAudioComponent.IsPlaying` _fmodaudio))
  (if _returnvalue
    (`/Engine/EditorBlueprintResources/StandardMacros.IsValid` _vis_wav_file
      (:`Is Valid`
        (bind _returnvalue_2 (`FMODAudioComponent.GetTimelinePosition` _fmodaudio))
        (bind _outamplitudes (`SoundVisualizationStatics.GetAmplitude` _vis_wav_file 0 (+ (mod (/ (`KismetMathLibrary.Conv_IntToDouble` _returnvalue_2) 1000.0) (`SoundBase.Duration` _vis_wav_file)) (`self.Time Adjustment`)) (`self.Sample Lenght`) 1))
        (set `self.Amplitude` (/ (`KismetArrayLibrary.Array_Get` _outamplitudes) (`self.AmplitudeDivide`)))))))