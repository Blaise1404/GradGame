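; A configurable object actor that ties a skeletal mesh's color to the pitch of an FMOD sound through a shared Hue value.
; The construction script applies the chosen mesh, creates a dynamic material instance and assigns the FMOD event.
; ChangeHue adds a hundredth of its input to Hue, then updates the material's Hue and the FMOD pitch parameter, wrapped to 0–1.
; PlayFMod plays the sound on demand.
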(fn `ChangeHue`
  (params (Value :type "Float (double-precision)"))
  (bind _output_get (set `self.Hue` (+ (stale _output_get) (/ Value 100.0))))
  (`self.UpdateColors`)
  (`self.UpdateFmod` 0))

(fn `PlayFMod`
  (`FMODAudioComponent.Play` (`self.FMODAudio`)))

(fn `UpdateColors`
  (`MaterialInstanceDynamic.SetScalarParameterValue` (`self.MaterialDynamic`) "Hue" (`self.Hue`)))

(fn `UpdateFmod`
  (params (ID :type Integer))
  (returns (Result :type Boolean))
  (`FMODAudioComponent.SetParameter` (`self.FMODAudio`) "Pitch -L" (mod (`self.Hue`) 1.0))
  (return true))

(fn `UserConstructionScript`
  (`|ExecutionSequence`
    (:`then_0`
      (`SkinnedMeshComponent.SetSkinnedAssetAndUpdate` (`self.SkeletalMesh`) (`self.Mesh`)))
    (:`then_1`
      (bind _returnvalue (`KismetMaterialLibrary.CreateDynamicMaterialInstance` (`self.Material`)))
      (bind _output_get (set `self.MaterialDynamic` _returnvalue))
      (`PrimitiveComponent.SetMaterial` (`self.SkeletalMesh`) 0 _output_get)
      (`self.UpdateColors`))
    (:`then_2`
      (`FMODAudioComponent.SetEvent` (`self.FMODAudio`) (`self.FModEvent`))
      (`self.UpdateFmod` 0))))