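; Background cone actor that continuously animates the U and V parameters of its static mesh material.
; The construction script creates and stores a dynamic material instance from the mesh's first material slot.
; On BeginPlay a timeline drives both scalar parameters each update, then restarts itself from the start through a PlayAgain event whenever it finishes, forming an endless loop.
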(event `self.ReceiveBeginPlay`
  (bind _material (`self.Material`))
  (bind (_direction _u _v) (`Timeline|Timeline_0` :!label _label)
    (:`Update`
      (`MaterialInstanceDynamic.SetScalarParameterValue` _material "U" _u)
      (`MaterialInstanceDynamic.SetScalarParameterValue` _material "V" _v))
    (:`Finished`
      (`self.PlayAgain`))))

(event `PlayAgain`
  (goto _label :!via `PlayFromStart`))

(fn `UserConstructionScript`
  (bind _staticmesh (`self.StaticMesh`))
  (bind _returnvalue (`PrimitiveComponent.CreateDynamicMaterialInstance` _staticmesh 0 (`PrimitiveComponent.GetMaterial` _staticmesh 0)))
  (set `self.Material` _returnvalue))