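; VR intro actor that teaches the grab, pull, edit and push gestures on a practice object, then opens the experience.
; An IntroStage machine advances on trigger input, VR_Character state changes and shape/hue edits, updating text above both controllers.
; The object smoothly follows state-driven targets, feeding edits to materials and FMOD.
; Completion plays a timeline that opens the cave and activates InteractiveObjects; after a fixed delay, End reverses it for credits and reset.
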(event `Key|MotionController_Left_Trigger` :consume false
  (params (Key :type "Key Structure" :default "AnyKey"))
  (bind _returnvalue (`KismetTextLibrary.Conv_StringToText` (`KismetStringLibrary.Concat_StrStr` "While pointing at object  <br> press THUMBSTICK to grab it")))
  (:`Pressed`
    (switch `int` (`self.IntroStage`) :!label _label
      (:`0`
        (`TextRenderComponent.K2_SetText` (`self.TextL`) _returnvalue)
        (`TextRenderComponent.K2_SetText` (`self.TextR`) _returnvalue)
        (set `self.IntroStage` 1)))))

(event `Key|MotionController_Right_Trigger` :consume false
  (params (Key :type "Key Structure" :default "AnyKey"))
  (:`Pressed`
    (goto _label)))

(event `Do Push`
  (bind _returnvalue (`KismetTextLibrary.Conv_StringToText` (`KismetStringLibrary.Concat_StrStr` "put hand inside then <br> press THUMBSTICK <br> to move it around")))
  (`TextRenderComponent.K2_SetText` (`self.TextL`) _returnvalue)
  (`TextRenderComponent.K2_SetText` (`self.TextR`) _returnvalue)
  (set `self.IntroStage` 5))

(event `IntroReact`
  (params (L :type "/Game/Blueprints/Controller/EControllerState Enum") (R :type "/Game/Blueprints/Controller/EControllerState Enum"))
  (bind _flower_cave (`self.flower_cave`))
  (bind _returnvalue (`KismetTextLibrary.Conv_StringToText` (`KismetStringLibrary.Concat_StrStr` "take it above your head <br>to put it back")))
  (bind _returnvalue_2 (`KismetTextLibrary.Conv_StringToText` (`KismetStringLibrary.Concat_StrStr` "to change it<br>put your hand inside <br> then press and hold TRIGGER <br> then pull the hand out")))
  (bind _returnvalue_3 (`KismetTextLibrary.Conv_StringToText` (`KismetStringLibrary.Concat_StrStr` "Move hand above your head <bt>to bring it close")))
  (bind _returnvalue_4 (`KismetTextLibrary.Conv_StringToText` (`KismetStringLibrary.Concat_StrStr` "")))
  (switch `int` (`self.IntroStage`)
    (:`1`
      (`|ExecutionSequence`
        (:`then_0`
          (switch `/Game/Blueprints/Controller/EControllerState` L
            (:`NewEnumerator2`
              _)))
        (:`then_1`
          (switch `/Game/Blueprints/Controller/EControllerState` R
            (:`NewEnumerator2`
              _))))
      (`TextRenderComponent.K2_SetText` (`self.TextL`) _returnvalue_3)
      (`TextRenderComponent.K2_SetText` (`self.TextR`) _returnvalue_3)
      (set `self.IntroStage` 2))
    (:`2`
      (`|ExecutionSequence`
        (:`then_0`
          (switch `/Game/Blueprints/Controller/EControllerState` L
            (:`NewEnumerator3`
              _)))
        (:`then_1`
          (switch `/Game/Blueprints/Controller/EControllerState` R
            (:`NewEnumerator3`
              _))))
      (`TextRenderComponent.K2_SetText` (`self.TextL`) _returnvalue_2)
      (`TextRenderComponent.K2_SetText` (`self.TextR`) _returnvalue_2)
      (set `self.IntroStage` 3))
    (:`3`
      (`|ExecutionSequence`
        (:`then_0`
          (switch `/Game/Blueprints/Controller/EControllerState` L
            (:`NewEnumerator11`
              _)))
        (:`then_1`
          (switch `/Game/Blueprints/Controller/EControllerState` R
            (:`NewEnumerator11`
              _))))
      (`TextRenderComponent.K2_SetText` (`self.TextL`) (`KismetTextLibrary.Conv_StringToText` (`KismetStringLibrary.Concat_StrStr` "this hand change SHAPE")))
      (`TextRenderComponent.K2_SetText` (`self.TextR`) (`KismetTextLibrary.Conv_StringToText` (`KismetStringLibrary.Concat_StrStr` "this hand change COLOR")))
      (set `self.IntroStage` 4))
    (:`5`
      (`|ExecutionSequence`
        (:`then_0`
          (switch `/Game/Blueprints/Controller/EControllerState` L
            (:`NewEnumerator4`
              _)))
        (:`then_1`
          (switch `/Game/Blueprints/Controller/EControllerState` R
            (:`NewEnumerator4`
              _))))
      (`TextRenderComponent.K2_SetText` (`self.TextL`) _returnvalue)
      (`TextRenderComponent.K2_SetText` (`self.TextR`) _returnvalue)
      (set `self.IntroStage` 6))
    (:`6`
      (`|ExecutionSequence`
        (:`then_0`
          (switch `/Game/Blueprints/Controller/EControllerState` L
            (:`NewEnumerator0`
              _)))
        (:`then_1`
          (switch `/Game/Blueprints/Controller/EControllerState` R
            (:`NewEnumerator0`
              _))))
      (`TextRenderComponent.K2_SetText` (`self.TextL`) _returnvalue_4)
      (`TextRenderComponent.K2_SetText` (`self.TextR`) _returnvalue_4)
      (set `self.IntroStage` 7)
      (`self.Activation` false)
      (bind (_direction _opacitylogo _emmisive _opacityoutside _logodown _credits) (`Timeline|Timeline_0` :!label _label_2)
        (:`Update`
          (`|ExecutionSequence`
            (:`then_0`
              (switch `ETimelineDirection` _direction
                (:`Forward`
                  (for _array_element (`self.MaterialsDynamic`)
                    (`MaterialInstanceDynamic.SetScalarParameterValue` _array_element "Emmisive" _emmisive)
                    (`MaterialInstanceDynamic.SetScalarParameterValue` _array_element "Opacity" _opacitylogo)))
                (:`Backward`
                  (`SceneComponent.K2_SetWorldLocation` (`self.Credits`) (`KismetMathLibrary.MakeVector` 0.0 0.0 _credits) false false))))
            (:`then_1`
              (`MaterialInstanceDynamic.SetScalarParameterValue` (`self.OutsideMat`) "Opacity" _opacityoutside)
              (if (`self.GoDown`)
                (`SceneComponent.K2_SetWorldLocation` (`self.SkeletalMesh`) (+ (`self.Position`) (`KismetMathLibrary.MakeVector` 0.0 0.0 _logodown)) false false)))))
        (:`OpenCave`
          (`SkeletalMeshComponent.Play` (`self.flower_cave`) false)
          (`FMODAudioComponent.Play` (`self.CaveOpen`)))
        (:`ActivateStars`
          (bind _outactors (`GameplayStatics.GetAllActorsOfClass` "/Game/Blueprints/Object/InteractiveObject.InteractiveObject_C"))
          (for _array_element_2 _outactors
            (`self.Activation` _array_element_2 true)))
        (:`GoDown`
          (set `self.Position` (`SceneComponent.K2_GetComponentLocation` (`self.SkeletalMesh`)))
          (set `self.GoDown` true)
          (`self.UpdateState` "NewEnumerator0"))
        (:`Close Cave`
          (switch `ETimelineDirection` _direction
            (:`Backward`
              (`SkeletalMeshComponent.SetPlayRate` _flower_cave -1.0)
              (`SkeletalMeshComponent.Play` _flower_cave false)
              (`FMODAudioComponent.Play` (`self.CaveClose`)))))))))

(event `self.ReceiveBeginPlay`
  ;[1 1 1] Begin Play
  (`|ExecutionSequence`
    (:`then_0`
      (bind _asvr_character (cast `/Game/Blueprints/VR_Character` (`GameplayStatics.GetPlayerCharacter` 0)))
      (set `self.ControllerL` (`/Game/Blueprints/VR_Character.Mesh_L` _asvr_character))
      (set `self.ControllerR` (`/Game/Blueprints/VR_Character.Mesh_R` _asvr_character))
      (add `/Game/Blueprints/VR_Character.ControllerStateChanged` _asvr_character (delegate `IntroReact`)))
    (:`then_1`
      (`self.Activation` true)
      (bind _returnvalue (`KismetMaterialLibrary.CreateDynamicMaterialInstance` (`PrimitiveComponent.GetMaterial` (`self.Outside`) 0)))
      (bind _output_get (set `self.OutsideMat` _returnvalue))
      (`PrimitiveComponent.SetMaterial` (`self.Outside`) 0 _output_get))
    (:`then_2`
      (`KismetSystemLibrary.Delay` 360.0)
      (`self.End`))
    (:`then_3`
      (`FMODAudioComponent.SetParameter` (`self.CaveOpen`) "0" 1.12)
      (`FMODAudioComponent.SetParameter` (`self.CaveClose`) "0" 1.26))))

(event `End`
  (bind _asvr_character (cast `/Game/Blueprints/VR_Character` (`GameplayStatics.GetPlayerCharacter` 0) :!pure true))
  (`|ExecutionSequence`
    (:`then_0`
      (`/Game/Blueprints/VR_Character.ChangeControllersState` _asvr_character "NewEnumerator0" "NewEnumerator10")
      (`/Game/Blueprints/VR_Character.ChangeControllersState` _asvr_character "NewEnumerator1" "NewEnumerator10")
      (goto _label_2 :!via `Reverse`))
    (:`then_1`
      (bind _outactors (`GameplayStatics.GetAllActorsOfClass` "/Game/Blueprints/Object/InteractiveObject.InteractiveObject_C"))
      (for _array_element _outactors
        (`self.Activation` _array_element false)
        (`self.UpdateState` _array_element "NewEnumerator0"))
      (`self.Activation` true))
    (:`then_2`
      (bind _outactors_2 (`GameplayStatics.GetAllActorsOfClass` "/Game/Blueprints/Level3/Objects/InstrumentPlanet.InstrumentPlanet_C"))
      (for _array_element_2 _outactors_2
        (`/Game/Blueprints/Object/Instrument.GoBack` _array_element_2)))))

(event `self.ReceiveTick`
  (params (DeltaSeconds :type "Float (single-precision)"))
  ;[1 1 1] Event Tick
  (`self.FollowControllers`)
  (switch `/Game/Blueprints/Object/EObjectTarget` (`self.State`)
    (:`NewEnumerator6`
      (if (>= (`self.IntroStage`) 7)
        (`self.SmoothFollow` (`self.SkeletalMesh`) (`self.CurrentTarget`) true :!label _label_3)))
    (:`NewEnumerator2`
      (goto _label_3))
    (:`NewEnumerator3`
      (if (< (`self.IntroStage`) 5) :!label _label_4
        (`self.UpdateState` "NewEnumerator2")
        (else
          (`self.SmoothFollow` (`self.SkeletalMesh`) (`self.CurrentTarget`)))))
    (:`NewEnumerator5`
      (goto _label_4))))

(event `self.PullUpdate`
  (params (Value :type "Float (single-precision)"))
  ;[1 1 1] Pull
  (switch `/Game/Blueprints/Object/EObjectTarget` (`self.State`)
    (:`NewEnumerator6`
      (if (> Value 0.9)
        (bind _asvr_character (cast `/Game/Blueprints/VR_Character` (`GameplayStatics.GetPlayerCharacter` 0)))
        (`/Game/Blueprints/VR_Character.PullSucces` _asvr_character)))))

(event `self.ChangeShape`
  (params (Value :type "Float (single-precision)") (Add :type "Float (single-precision)"))
  (bind _returnvalue (+ Value (* (`KismetMathLibrary.Abs` Add) 1.3)))
  ;[1 1 1] Edit
  (if (`self.ShapeDone`)
    _
    (elif (>= _returnvalue 1.0)
      (set `self.ShapeDone` true)
      (`TextRenderComponent.K2_SetText` (`self.TextL`) (`KismetTextLibrary.Conv_StringToText` (`KismetStringLibrary.Concat_StrStr` "")))
      (if (`self.HueDone`)
        (`self.Do Push` :!label _label_5))
      (else
        (bind _output_get (set `self.Shape` _returnvalue))
        (`self.UpdateFmod` "1" _output_get)
        (`self.UpdateShape` 0.0)))))

(event `self.ChangeHue`
  (params (Value :type "Float (single-precision)") (Add :type "Float (single-precision)"))
  (bind _returnvalue (+ Value (* (`KismetMathLibrary.Abs` Add) 1.3)))
  ;[1 1 1] Edit
  (if (`self.HueDone`)
    _
    (elif (>= _returnvalue 1.0)
      (set `self.HueDone` true)
      (`TextRenderComponent.K2_SetText` (`self.TextR`) (`KismetTextLibrary.Conv_StringToText` (`KismetStringLibrary.Concat_StrStr` "")))
      (if (`self.ShapeDone`)
        (goto _label_5))
      (else
        (bind _output_get (set `self.Hue` _returnvalue))
        (`self.UpdateColors`)
        (`self.UpdateFmod` "0" _output_get)
        (for _array_element (`self.MaterialsDynamic`)
          (`MaterialInstanceDynamic.SetScalarParameterValue` _array_element "Saturation" (`KismetMathLibrary.FClamp` (`self.Hue`)))
          (`MaterialInstanceDynamic.SetScalarParameterValue` _array_element "Emmisive" (`KismetMathLibrary.FClamp` (+ (* (`self.Hue`) 7.0) 0.7) 0.0 7.5)))))))

(event `self.PushEnd`
  (params (GoBack :type Boolean))
  (if GoBack
    (switch `/Game/Blueprints/Object/EObjectTarget` (`self.State`)
      (:`NewEnumerator3`
        _)
      (:`NewEnumerator5`
        _))
    (`self.UpdateState` "NewEnumerator6")
    (else
      (`self.UpdateState` "NewEnumerator2"))))

(event `self.UpdateState`
  (params (State :type "/Game/Blueprints/Object/EObjectTarget Enum" :default "NewEnumerator0"))
  (bind _data (`self.Data`))
  (switch `/Game/Blueprints/Object/EObjectTarget` State
    (:`NewEnumerator0`
      (set `self.CurrentTarget` (`self.OrbitTarget`))
      (switch `/Game/Blueprints/Object/EObjectTarget` (`self.State`)
        (:`NewEnumerator0`
          (set `self.FollowSpeed` 2.0 :!label _label_6))
        (:`NewEnumerator6`
          (goto _label_6))
        (:`NewEnumerator1`
          (set `self.FollowSpeed` 0.4))
        (:`NewEnumerator2`
          (goto _label_6))
        (:`NewEnumerator3`
          (set `self.FollowSpeed` 2.0 :!label _label_7))
        (:`NewEnumerator5`
          (goto _label_7))))
    (:`NewEnumerator6`
      (set `self.CurrentTarget` (`self.TempTarget`)))
    (:`NewEnumerator1`
      (set `self.CurrentTarget` (`/Game/Blueprints/GameSettings/DATA.Target1` _data)))
    (:`NewEnumerator2`
      (set `self.CurrentTarget` (`/Game/Blueprints/GameSettings/DATA.Target2` _data))
      (set `self.FollowSpeed` 1.0))
    (:`NewEnumerator3`
      (set `self.CurrentTarget` (`/Game/Blueprints/GameSettings/DATA.TargetL` _data)))
    (:`NewEnumerator5`
      (set `self.CurrentTarget` (`/Game/Blueprints/GameSettings/DATA.TargetR` _data))))
  (set `self.State` State))

(fn `FollowControllers`
  (bind _controllerr (`self.ControllerR`))
  (bind _controllerl (`self.ControllerL`))
  (bind _textr (`self.TextR`))
  (bind _textl (`self.TextL`))
  (bind (_returnvalue_roll _returnvalue_pitch _returnvalue_yaw) (`KismetMathLibrary.BreakRotator` (`SceneComponent.K2_GetComponentRotation` _controllerr)))
  (bind (_returnvalue_roll_2 _returnvalue_pitch_2 _returnvalue_yaw_2) (`KismetMathLibrary.BreakRotator` (`SceneComponent.K2_GetComponentRotation` _controllerl)))
  (`|ExecutionSequence`
    (:`then_0`
      (`SceneComponent.K2_SetWorldLocation` _textr (+ (`SceneComponent.K2_GetComponentLocation` _controllerr) (0.0 0.0 15.0)) false false)
      (`SceneComponent.K2_SetWorldRotation` _textr (`KismetMathLibrary.MakeRotator` 0.0 0.0 (+ _returnvalue_yaw 180.0)) false false))
    (:`then_1`
      (`SceneComponent.K2_SetWorldLocation` _textl (+ (`SceneComponent.K2_GetComponentLocation` _controllerl) (0.0 0.0 15.0)) false false)
      (`SceneComponent.K2_SetWorldRotation` _textl (`KismetMathLibrary.MakeRotator` 0.0 0.0 (+ _returnvalue_yaw_2 180.0)) false false))))

(fn `SmoothFollow`
  (params (Object :type "SceneComponent Object Reference") (Target :type "SceneComponent Object Reference") (`With Scale` :type Boolean))
  (returns (Dummy :type Boolean))
  (bind (_returnvalue_location _returnvalue_rotation _returnvalue_scale) (`KismetMathLibrary.BreakTransform` (`SceneComponent.K2_GetComponentToWorld` Object)))
  (bind _returnvalue (`GameplayStatics.GetWorldDeltaSeconds`))
  (bind (_returnvalue_location_2 _returnvalue_rotation_2 _returnvalue_scale_2) (`KismetMathLibrary.BreakTransform` (`SceneComponent.K2_GetComponentToWorld` Target)))
  (bind _followspeed (`self.FollowSpeed`))
  (`SceneComponent.K2_SetWorldLocation` Object (`KismetMathLibrary.VInterpTo` _returnvalue_location _returnvalue_location_2 _returnvalue _followspeed) false false)
  (`SceneComponent.K2_SetWorldRotation` Object (`KismetMathLibrary.RInterpTo` _returnvalue_rotation _returnvalue_rotation_2 _returnvalue _followspeed) false false)
  (if `With Scale`
    (`SceneComponent.SetWorldScale3D` Object (`KismetMathLibrary.VInterpTo` _returnvalue_scale _returnvalue_scale_2 _returnvalue _followspeed)))
  (return false))

(fn `UserConstructionScript`
  (`|ExecutionSequence`
    (:`then_0`
      (`SkinnedMeshComponent.SetSkinnedAssetAndUpdate` (`self.SkeletalMesh`) (`self.Mesh`) true))
    (:`then_1`
      (for (_array_element _array_index) (`self.Materials`)
        (bind _returnvalue (`KismetMaterialLibrary.CreateDynamicMaterialInstance` _array_element))
        (`KismetArrayLibrary.Array_Set` (`self.MaterialsDynamic`) _array_index _returnvalue true)
        (`PrimitiveComponent.SetMaterial` (`self.SkeletalMesh`) _array_index _returnvalue)))
    (:`then_2`
      (`FMODAudioComponent.SetEvent` (`self.FMODAudio`) (`self.Fmod Event`)))
    (:`then_3`
      (`self.UpdateColors`))))