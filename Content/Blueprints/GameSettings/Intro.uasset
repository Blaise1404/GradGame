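; VR intro object, an InteractiveObject child, that teaches grabbing, pulling, twisting and throwing before opening the main experience.
; IntroStage advances through trigger and interaction events, updating hint texts that follow both controllers.
; Maxing shape and hue leads to the throw, where Start plays a timeline opening the cave and activating other InteractiveObjects and NoiseSpawn.
; After a Playtime delay from first trigger press, End reverses that timeline, showing credits and deactivating those objects.
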(event `Key|MotionController_Left_Trigger` :consume false
  (params (Key :type "Key Structure" :default "AnyKey"))
  (bind _returnvalue (`KismetTextLibrary.Conv_StringToText` "Point at object <br> to grab it"))
  ;[1 1 1] State switch
  (:`Pressed`
    (switch `int` (`self.IntroStage`) :!label _label
      (:`0`
        (`TextRenderComponent.K2_SetText` (`self.TextL`) _returnvalue)
        (`TextRenderComponent.K2_SetText` (`self.TextR`) _returnvalue)
        (set `self.IntroStage` 1)
        (`KismetSystemLibrary.Delay` (`self.Playtime`))
        (`self.End`))
      (:`3`
        (`TextRenderComponent.K2_SetText` (`self.TextL`) (`KismetTextLibrary.Conv_StringToText` (`KismetStringLibrary.Concat_StrStr` "TWIST  this hand<br>to change SHAPE")))
        (`TextRenderComponent.K2_SetText` (`self.TextR`) (`KismetTextLibrary.Conv_StringToText` (`KismetStringLibrary.Concat_StrStr` "TWIST this hand<br>to change COLOR")))
        (`SceneComponent.SetRelativeScale3D` (`self.OrbitTarget`) (0.6 0.6 0.6))
        (set `self.IntroStage` 4)))))

(event `Key|MotionController_Right_Trigger` :consume false
  (params (Key :type "Key Structure" :default "AnyKey"))
  ;[1 1 1] State switch
  (:`Pressed`
    (goto _label)))

(event `self.ReceiveBeginPlay`
  ;[1 1 1] Begin Play
  (`parent.ReceiveBeginPlay`)
  (`|ExecutionSequence`
    (:`then_0`
      (bind _output_get (set `self.InitialHue` (`KismetMathLibrary.RandomFloatInRange` 0.0 1.0)))
      (`MaterialInstanceDynamic.SetScalarParameterValue` (`KismetArrayLibrary.Array_Get` (`self.MaterialsDynamic`) 1) "Hue" _output_get))
    (:`then_1`
      (`self.Activation` true)
      (`self.PlayFMod`)
      (bind _returnvalue (`KismetMaterialLibrary.CreateDynamicMaterialInstance` (`PrimitiveComponent.GetMaterial` (`self.Outside`) 0)))
      (bind _output_get_2 (set `self.OutsideMat` _returnvalue))
      (`PrimitiveComponent.SetMaterial` (`self.Outside`) 0 _output_get_2))
    (:`then_2`
      (bind _asvr_character (cast `/Game/Blueprints/GameSettings/VR_Character` (`GameplayStatics.GetPlayerCharacter` 0)))
      (set `self.ControllerR` (`/Game/Blueprints/GameSettings/Controller/VRController.Controller Mesh` (`/Game/Blueprints/GameSettings/VR_Character.ControllerR` _asvr_character)))
      (set `self.ControllerL` (`/Game/Blueprints/GameSettings/Controller/VRController.Controller Mesh` (`/Game/Blueprints/GameSettings/VR_Character.ControllerL` _asvr_character))))))

(event `self.PullStart`
  ;[1 1 1] State switch
  (`parent.PullStart`)
  (if (== (`self.IntroStage`) 1)
    (`TextRenderComponent.K2_SetText` (`self.TextL`) (`KismetTextLibrary.Conv_StringToText` "Pull to bring it close"))
    (`TextRenderComponent.K2_SetText` (`self.TextR`) (`KismetTextLibrary.Conv_StringToText` "Pull to bring it close"))
    (set `self.ObjectOffset` (stale _output_get))
    (bind _output_get (set `/Game/Blueprints/GameSettings/VR_Character.ObjectTargetOffset` (60.0 0.0 -10.0) (cast `/Game/Blueprints/GameSettings/VR_Character` (`GameplayStatics.GetPlayerCharacter` 0) :!pure true)))
    (set `self.IntroStage` 2)))

(event `self.MoveDone`
  (params (Back :type Boolean))
  ;[1 1 1] State switch
  (switch `/Game/Blueprints/GeneralFunctions/EObjectTarget` (`self.State`)
    (:`NewEnumerator6`
      (if Back
        (`self.UpdateState` "NewEnumerator0")
        (else
          (`TextRenderComponent.K2_SetText` (`self.TextL`) (`KismetTextLibrary.Conv_StringToText` "Press and hold TRIGGER <br>to change it"))
          (`TextRenderComponent.K2_SetText` (`self.TextR`) (`KismetTextLibrary.Conv_StringToText` "Press and hold TRIGGER <br>to change it"))
          (set `self.IntroStage` 3)
          (`parent.MoveDone` false)
          (`PrimitiveComponent.SetCollisionObjectType` (`self.Collider`) "ECC_GameTraceChannel1"))))
    (:`NewEnumerator3`
      (if Back
        (`parent.MoveDone` true)
        (`self.Start`)
        (else
          (`parent.MoveDone` false))))))

(event `Do Push`
  ;[1 1 1] State switch
  (set `self.Radius` 990.0)
  (`TextRenderComponent.K2_SetText` (`self.TextL`) (`KismetTextLibrary.Conv_StringToText` (`KismetStringLibrary.Concat_StrStr` "Touch it and <br> hold TRIGGER <br> to grab it")))
  (`TextRenderComponent.K2_SetText` (`self.TextR`) (`KismetTextLibrary.Conv_StringToText` (`KismetStringLibrary.Concat_StrStr` "Touch it and <br> hold TRIGGER <br> to grab it")))
  (`PrimitiveComponent.SetCollisionObjectType` (`self.Collider`) "ECC_WorldDynamic")
  (set `self.IntroStage` 5))

(event `self.SmoothFollow`
  (params (Object :type "SceneComponent Object Reference") (Target :type "SceneComponent Object Reference") (Scale :type Boolean) (Rotation :type Boolean))
  ;[1 1 1] Smooth Follow
  (`parent.SmoothFollow` Object Target Scale (`self.FollowRot`)))

(event `self.ReceiveTick`
  (params (DeltaSeconds :type "Float (single-precision)"))
  ;[1 1 1] Event Tick
  (`parent.ReceiveTick` DeltaSeconds)
  (`self.FollowControllers`)
  (if (`|EnumEquality` (`self.State`) "NewEnumerator6")
    (`SceneComponent.K2_SetWorldRotation` (`self.TempTarget`) (`SceneComponent.K2_GetComponentRotation` (`self.OrbitTarget`)) false false)))

(event `self.MoveStart`
  (params (Controller :type "/Game/Blueprints/GameSettings/Controller/VRController Object Reference"))
  (bind _orbittarget (`self.OrbitTarget`))
  ;[1 1 1] State switch
  (`parent.MoveStart` Controller)
  (`TextRenderComponent.K2_SetText` (`self.TextL`) (`KismetTextLibrary.Conv_StringToText` (`KismetStringLibrary.Concat_StrStr` "Throw it up<br>to put it back")))
  (`TextRenderComponent.K2_SetText` (`self.TextR`) (`KismetTextLibrary.Conv_StringToText` (`KismetStringLibrary.Concat_StrStr` "Throw it up<br>to put it back")))
  (set `self.IntroStage` 6)
  (`SceneComponent.K2_SetWorldRotation` (`self.TempTarget`) (`SceneComponent.K2_GetComponentRotation` _orbittarget) false false)
  (`SceneComponent.K2_SetWorldRotation` _orbittarget (struct :`Yaw` 24.0) false false))

(event `Start`
  (bind _cave (`self.Cave`))
  (bind _flower_cave (`self.flower_cave`))
  ;[1 1 1] State switch
  (`|ExecutionSequence`
    (:`then_0`
      (set `/Game/Blueprints/GameSettings/VR_Character.ObjectTargetOffset` (`self.ObjectOffset`) (cast `/Game/Blueprints/GameSettings/VR_Character` (`GameplayStatics.GetPlayerCharacter` 0) :!pure true))
      (`FMODAudioComponent.Play` (`self.Cave`)))
    (:`then_1`
      (set `self.FollowRot` true)
      (`TextRenderComponent.K2_SetText` (`self.TextL`) (`KismetTextLibrary.Conv_StringToText` ""))
      (`TextRenderComponent.K2_SetText` (`self.TextR`) (`KismetTextLibrary.Conv_StringToText` ""))
      (set `self.IntroStage` 7)
      (`self.Activation` false)
      (`SceneComponent.K2_AddWorldRotation` (`self.TempTarget`) (struct :`Yaw` 30.0) false false)
      (`ParticleSystemComponent.SetEmitterEnable` (`self.IntroLights`) "Lights" false)
      (bind _outactors (`GameplayStatics.GetAllActorsOfClass` "/Game/Blueprints/GameSettings/NoiseSpawn.NoiseSpawn_C"))
      (`/Game/Blueprints/GameSettings/NoiseSpawn.Start` (`KismetArrayLibrary.Array_Get` _outactors))
      (bind (_direction _opacitylogo _emmisive _opacityoutside _logodown _credits _instrumentpos) (`Timeline|Timeline_0` :!label _label_2)
        (:`Update`
          (`|ExecutionSequence`
            (:`then_0`
              (switch `ETimelineDirection` _direction
                (:`Forward`
                  (for _array_element (`self.MaterialsDynamic`)
                    (`MaterialInstanceDynamic.SetScalarParameterValue` _array_element "Emmisive" _emmisive)
                    (`MaterialInstanceDynamic.SetScalarParameterValue` _array_element "Opacity" _opacitylogo)))
                (:`Backward`
                  (`SceneComponent.K2_SetWorldLocation` (`self.Credits`) (`KismetMathLibrary.MakeVector` 0.0 0.0 _credits) false false)
                  (`SceneComponent.SetRelativeScale3D` (`/Game/Blueprints/GameSettings/VR_Character.InstrumentCentre` (cast `/Game/Blueprints/GameSettings/VR_Character` (`GameplayStatics.GetPlayerCharacter` 0) :!pure true)) (`KismetMathLibrary.Conv_DoubleToVector` _instrumentpos)))))
            (:`then_1`
              (`MaterialInstanceDynamic.SetScalarParameterValue` (`self.OutsideMat`) "Opacity" _opacityoutside)
              (if (`self.GoDown`)
                (`SceneComponent.K2_SetRelativeLocation` (`self.Object`) (+ (`self.Position`) (`KismetMathLibrary.MakeVector` 0.0 0.0 _logodown)) false false)))))
        (:`Finished`
          (set `self.CurrentTarget` null)
          (switch `ETimelineDirection` _direction))
        (:`OpenCave`
          (switch `ETimelineDirection` _direction
            (:`Forward`
              (`SkeletalMeshComponent.Play` (`self.flower_cave`) false)
              (`SceneComponent.SetHiddenInGame` (`self.work in progress`) false false))))
        (:`ActivateStars`
          (switch `ETimelineDirection` _direction
            (:`Forward`
              (bind _outactors_2 (`GameplayStatics.GetAllActorsOfClass` "/Game/Blueprints/ObjectsBase/InteractiveObject.InteractiveObject_C"))
              (`|ExecutionSequence`
                (:`then_0`
                  (for _array_element_2 _outactors_2
                    (if (!= _array_element_2 self)
                      (`self.Activation` _array_element_2 true)
                      (`self.PlayFMod` _array_element_2))))
                (:`then_1`
                  (bind _outactors_3 (`GameplayStatics.GetAllActorsOfClass` "/Game/Blueprints/GameSettings/NoiseSpawn.NoiseSpawn_C"))
                  (bind _output_get (set `self.NoiseSpawn` (`KismetArrayLibrary.Array_Get` _outactors_3)))
                  (bind (_item_noiseclass _item_delay) (break `/Game/Blueprints/GeneralFunctions/NoiseDetalis` (`KismetArrayLibrary.Array_Get` (`/Game/Blueprints/GameSettings/NoiseSpawn.Noises` _output_get))))
                  (`KismetSystemLibrary.Delay` _item_delay)
                  (`/Game/Blueprints/GameSettings/NoiseSpawn.Start` _output_get))))))
        (:`GoDown`
          (set `self.Position` (`SceneComponent.RelativeLocation` (`self.Object`)))
          (set `self.GoDown` true))
        (:`Close Cave`
          (switch `ETimelineDirection` _direction
            (:`Backward`
              (`FMODAudioComponent.SetParameter` _cave "0" 1.0)
              (`FMODAudioComponent.Play` _cave)
              (`SkeletalMeshComponent.SetPlayRate` _flower_cave -1.0)
              (`SkeletalMeshComponent.Play` _flower_cave false)
              (`ParticleSystemComponent.SetEmitterEnable` (`self.IntroLights`) "Lights" true)
              (`/Game/Blueprints/GameSettings/NoiseSpawn.Stop` (`self.NoiseSpawn`))
              (bind (_direction_2 _newtrack_0) (`Timeline|Logolayers`)
                (:`Update`
                  (`FMODAudioComponent.SetParameter` (`self.FMODAudio`) "1" _newtrack_0))))))
        (:`LogoStop`
          (switch `ETimelineDirection` _direction
            (:`Forward`
              (`FMODAudioComponent.Stop` (`self.FMODAudio`)))))))))

(event `End`
  (bind (_returnvalue_roll _returnvalue_pitch _returnvalue_yaw) (`KismetMathLibrary.BreakRotator` (`SceneComponent.K2_GetComponentRotation` (`/Game/Blueprints/GameSettings/VR_Character.Camera` (cast `/Game/Blueprints/GameSettings/VR_Character` (`GameplayStatics.GetPlayerCharacter` 0) :!pure true)))))
  ;[1 1 1] State switch
  (`|ExecutionSequence`
    (:`then_0`
      (`SceneComponent.K2_SetWorldRotation` (`self.DefaultSceneRoot`) (`KismetMathLibrary.MakeRotator` 0.0 0.0 _returnvalue_yaw) false false))
    (:`then_1`
      (`/Game/Blueprints/GameSettings/Controller/VRController.StateChange` (`/Game/Blueprints/GameSettings/VR_Character.ControllerL` (cast `/Game/Blueprints/GameSettings/VR_Character` (`GameplayStatics.GetPlayerCharacter` 0) :!pure true)) "NewEnumerator10")
      (`/Game/Blueprints/GameSettings/Controller/VRController.StateChange` (`/Game/Blueprints/GameSettings/VR_Character.ControllerR` (cast `/Game/Blueprints/GameSettings/VR_Character` (`GameplayStatics.GetPlayerCharacter` 0) :!pure true)) "NewEnumerator10")
      (goto _label_2 :!via `Reverse`))
    (:`then_2`
      (bind _outactors (`GameplayStatics.GetAllActorsOfClass` "/Game/Blueprints/ObjectsBase/InteractiveObject.InteractiveObject_C"))
      (for _array_element _outactors
        (if (!= _array_element self)
          (`self.Activation` _array_element false)
          (`FMODAudioComponent.Stop` (`/Game/Blueprints/ObjectsBase/iObject.FMODAudio` _array_element))
          (`self.UpdateState` _array_element "NewEnumerator0" null)
          (else
            (`self.Activation` true)
            (`FMODAudioComponent.SetParameter` (`self.FMODAudio`) "1" 0.0)
            (`self.PlayFMod`)))))
    (:`then_3`
      (`SceneComponent.SetHiddenInGame` (`self.work in progress`) true false))))

(fn `ChangeHue`
  (params (Value :type "Float (double-precision)") (Add :type "Float (double-precision)"))
  (if (`self.HueDone`)
    (return)
    (else
      (bind _output_get (set `self.Hue` (`KismetMathLibrary.FClamp` (+ Value (* (`KismetMathLibrary.Abs` Add) 3.0)) 0.0 0.99)))
      (`self.UpdateColors`)
      (`self.UpdateFmod` "0" _output_get)
      (`|ExecutionSequence`
        (:`then_0`
          (for _array_element (`self.MaterialsDynamic`)
            (`MaterialInstanceDynamic.SetScalarParameterValue` _array_element "Saturation" (`self.Hue`))
            (`MaterialInstanceDynamic.SetScalarParameterValue` _array_element "Emmisive" (`KismetMathLibrary.FClamp` (* (`self.Hue`) 10.0) 0.7 10.0))))
        (:`then_1`
          (if (>= _output_get 0.99)
            (set `self.HueDone` true)
            (`TextRenderComponent.K2_SetText` (`self.TextR`) (`KismetTextLibrary.Conv_StringToText` "Now change shape to flat"))
            (if (`self.ShapeDone`)
              (`self.Do Push`))
            (return)
            (else
              (return))))))))

(fn `ChangeShape`
  (params (Value :type "Float (double-precision)") (Add :type "Float (double-precision)"))
  (if (`self.ShapeDone`)
    (return)
    (else
      (bind _output_get (set `self.Shape` (`KismetMathLibrary.FClamp` (+ Value (* (`KismetMathLibrary.Abs` Add) 3.0)) 0.0 0.99)))
      (`self.UpdateFmod` "1" _output_get)
      (`self.UpdateShape` 0.0)
      (if (>= _output_get 0.99)
        (set `self.ShapeDone` true)
        (`TextRenderComponent.K2_SetText` (`self.TextL`) (`KismetTextLibrary.Conv_StringToText` "Now change color to white"))
        (`self.UpdateFmod` "1" 0.95)
        (if (`self.HueDone`)
          (`self.Do Push`))
        (return)
        (else
          (return))))))

(fn `FollowControllers`
  (bind _controllerr (`self.ControllerR`))
  (bind _controllerl (`self.ControllerL`))
  (bind _textr (`self.TextR`))
  (bind _textl (`self.TextL`))
  (bind (_returnvalue_roll _returnvalue_pitch _returnvalue_yaw) (`KismetMathLibrary.BreakRotator` (`SceneComponent.K2_GetComponentRotation` _controllerr)))
  (bind (_returnvalue_roll_2 _returnvalue_pitch_2 _returnvalue_yaw_2) (`KismetMathLibrary.BreakRotator` (`SceneComponent.K2_GetComponentRotation` _controllerl)))
  (`|ExecutionSequence`
    (:`then_0`
      (`SceneComponent.K2_SetWorldLocation` _textr (+ (`SceneComponent.K2_GetComponentLocation` _controllerr) (0.0 0.0 10.0)) false false)
      (`SceneComponent.K2_SetWorldRotation` _textr (`KismetMathLibrary.MakeRotator` 0.0 0.0 (+ _returnvalue_yaw 180.0)) false false))
    (:`then_1`
      (`SceneComponent.K2_SetWorldLocation` _textl (+ (`SceneComponent.K2_GetComponentLocation` _controllerl) (0.0 0.0 10.0)) false false)
      (`SceneComponent.K2_SetWorldRotation` _textl (`KismetMathLibrary.MakeRotator` 0.0 0.0 (+ _returnvalue_yaw_2 180.0)) false false))))

(fn `UserConstructionScript`
  (`parent.UserConstructionScript`))