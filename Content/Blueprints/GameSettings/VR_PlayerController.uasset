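; VR player controller meant to route movement input to either a star or a block, though none of that logic is connected.
; Unwired graph fragments switch on ActiveObject to pass vertical and horizontal input and to toggle between the two targets.
; The construction script caches the first TestObject as the block reference; its BP_HotStar2_MyBlueprint search result goes unused.
; BeginPlay and Tick are empty.
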(event `self.ReceiveBeginPlay`)

(event `self.ReceiveTick`
  (params (DeltaSeconds :type "Float (single-precision)")))

(fn `UserConstructionScript`
  (bind _outactors (`GameplayStatics.GetAllActorsOfClass` "/Game/Blueprints/TestObject.TestObject_C"))
  (set `self.ObjectReference` (`KismetArrayLibrary.Array_Get` _outactors))
  (bind _outactors_2 (`GameplayStatics.GetAllActorsOfClass` "/Game/FXStarStarterKit/Blueprint/BP_HotStar2_MyBlueprint.BP_HotStar2_MyBlueprint_C")))