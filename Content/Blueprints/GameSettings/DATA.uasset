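; DATA is an actor that follows the VR player's camera location and yaw and holds shared references to the character, its targets and the level's instruments.
; BeginPlay caches the VR character, camera and left and right targets, fills an Instruments array indexed by each Instrument's ID, and sets a PullSuccessful parameter.
; Tick updates the transform from the camera.
; Overlap events are empty, and the InteractiveObject pull and push-back logic is disconnected.
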(event `self.ReceiveBeginPlay`
  (`|ExecutionSequence`
    (:`then_0`
      (bind _asvr_character (cast `/Game/Blueprints/VR_Character` (`GameplayStatics.GetPlayerCharacter` 0)))
      (set `self.VR Character` _asvr_character)
      (set `self.TargetL` (`/Game/Blueprints/VR_Character.TargetL` _asvr_character))
      (set `self.TargetR` (`/Game/Blueprints/VR_Character.TargetR` _asvr_character))
      (set `self.Camera` (`/Game/Blueprints/VR_Character.Camera` _asvr_character)))
    (:`then_1`
      (bind _outactors (`GameplayStatics.GetAllActorsOfClass` "/Game/Blueprints/Object/Instrument.Instrument_C"))
      (`KismetArrayLibrary.Array_Resize` (`self.Instruments`) (`KismetArrayLibrary.Array_Length` _outactors))
      (for _array_element _outactors
        (`KismetArrayLibrary.Array_Set` (`self.Instruments`) (`/Game/Blueprints/Object/Instrument.ID` _array_element) _array_element)))
    (:`then_2`
      (`FMODAudioComponent.SetParameter` (`self.PullSuccessful`) "0" 0.72))))

(event `self.ReceiveTick`
  (params (DeltaSeconds :type "Float (single-precision)"))
  (bind _returnvalue (`SceneComponent.K2_GetComponentToWorld` (`self.Camera`)))
  (`self.K2_SetActorTransform` (`KismetMathLibrary.MakeTransform` (.location _returnvalue) (`KismetMathLibrary.MakeRotator` 0.0 0.0 (.yaw (.rotation _returnvalue))))))

(event `self.Target1.OnComponentBeginOverlap`
  (params (OverlappedComponent :type "PrimitiveComponent Object Reference") (OtherActor :type "Actor Object Reference") (OtherComp :type "PrimitiveComponent Object Reference") (OtherBodyIndex :type Integer) (bFromSweep :type Boolean) (SweepResult :type "HitResult Structure (by ref)")))

(event `self.LeaveTarget.OnComponentBeginOverlap`
  (params (OverlappedComponent :type "PrimitiveComponent Object Reference") (OtherActor :type "Actor Object Reference") (OtherComp :type "PrimitiveComponent Object Reference") (OtherBodyIndex :type Integer) (bFromSweep :type Boolean) (SweepResult :type "HitResult Structure (by ref)")))

(fn `UserConstructionScript`)