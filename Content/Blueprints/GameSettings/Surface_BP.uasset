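; Surface_BP is a mesh surface actor whose material reacts to the VR character's amplitude sum, apparently as a visualizer.
; On BeginPlay it applies the first entry of its Materials array as a dynamic instance on the static mesh and caches the first VR_Character found in the level.
; Each Tick it writes the character's AmplitudesSum into the material's "Vis" scalar parameter.
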(event `self.ReceiveBeginPlay`
  (`self.ApplyMaterial` (`KismetArrayLibrary.Array_Get` (`self.Materials`)))
  (bind _outactors (`GameplayStatics.GetAllActorsOfClass` "/Game/Blueprints/GameSettings/VR_Character.VR_Character_C"))
  (set `self.Character` (`KismetArrayLibrary.Array_Get` _outactors)))

(event `self.ReceiveTick`
  (params (DeltaSeconds :type "Float (single-precision)"))
  (`MaterialInstanceDynamic.SetScalarParameterValue` (`self.Material`) "Vis" (`/Game/Blueprints/GameSettings/VR_Character.AmplitudesSum` (`self.Character`))))

(fn `ApplyMaterial`
  (params (Mat :type "MaterialInstance Object Reference"))
  (bind _returnvalue (`KismetMaterialLibrary.CreateDynamicMaterialInstance` Mat))
  (bind _output_get (set `self.Material` _returnvalue))
  (`PrimitiveComponent.SetMaterial` (`self.StaticMeshComponent`) 0 _output_get))

(fn `UserConstructionScript`)