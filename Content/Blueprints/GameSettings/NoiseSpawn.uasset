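; NoiseSpawn is a spawner actor that periodically creates noise actors suited to the VR character's active level.
; The construction script caches the first VR_Character, whose ActiveLevel indexes the Noises array for class and interval.
; Tick accumulates time and spawns when it exceeds that interval, scaled by a random variation re-rolled after each spawn.
; Start enables ticking, while Stop calls Destroyed on every Noise actor and disables ticking.
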(event `self.ReceiveBeginPlay`)

(event `Start`
  (`self.SetActorTickEnabled` true))

(event `self.ReceiveTick`
  (params (DeltaSeconds :type "Float (single-precision)"))
  (bind (_item_noiseclass _item_delay _item_interval) (break `/Game/Blueprints/GeneralFunctions/NoiseDetalis` (`KismetArrayLibrary.Array_Get` (`self.Noises`) (`/Game/Blueprints/GameSettings/VR_Character.ActiveLevel` (`self.Character`)))))
  (bind _output_get (set `self.Timer` (+ (stale _output_get) DeltaSeconds)))
  (if (> _output_get (* _item_interval (`self.Variation`)))
    (set `self.Timer` 0.0)
    (bind _returnvalue (`|SpawnActorFromClass` _item_noiseclass (`KismetMathLibrary.MakeTransform` (0.0 0.0 0.0)) "AlwaysSpawn" "OverrideRootScale"))
    (set `self.LatestNoise` _returnvalue)
    (set `self.Variation` (`KismetMathLibrary.RandomFloatInRange` 0.8 1.2))))

(event `Stop`
  (bind _outactors (`GameplayStatics.GetAllActorsOfClass` "/Game/Blueprints/ObjectsBase/Noise.Noise_C"))
  (for _array_element _outactors
    (`/Game/Blueprints/ObjectsBase/Noise.Destroyed` _array_element))
  (`self.SetActorTickEnabled` false))

(fn `SpawnNoise`)

(fn `UserConstructionScript`
  (bind _outactors (`GameplayStatics.GetAllActorsOfClass` "/Game/Blueprints/GameSettings/VR_Character.VR_Character_C"))
  (set `self.Character` (`KismetArrayLibrary.Array_Get` _outactors)))