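; VR player character for a game with instruments: sets up the HMD, indexes Instrument actors by ID and forwards trigger presses to both motion controllers.
; Each tick, the instrument belt and active object's close target follow camera position and yaw, and amplitudes are summed.
; A reversible timeline in MoveBelt shifts the belt's height and scale.
; Temporary keyboard and mouse controls support testing, including hue/shape changes and camera rotation.
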(event `Key|MotionController_Right_Thumbstick`
  (params (Key :type "Key Structure" :default "LeapLeftPinch"))
  ;[1 0 0.07764] Temp
)

(event `Key|MotionController_Left_Thumbstick`
  (params (Key :type "Key Structure" :default "LeapLeftPinch"))
  ;[1 0 0.07764] Temp
)

(event `Keyboad Control`
  (bind _controllerl (`self.ControllerL`))
  (bind _controllerr (`self.ControllerR`))
  (bind _activeobject (`self.ActiveObject`))
  (bind _activeobject_2 (`self.ActiveObject`))
  (bind _activeobject_3 (`self.ActiveObject`))
  (bind _activeobject_4 (`self.ActiveObject`))
  ;[1 0 0.7382] REMOVE
  (`|ExecutionSequence`
    (:`then_0`
      (if (`self.Left Pressed`)
        (`/Engine/EditorBlueprintResources/StandardMacros.IsValid` _controllerl
          (:`Is Valid`
            (if (== _activeobject_3 null)
              (`/Game/Blueprints/ObjectsBase/iObject.ChangeHue` _activeobject_3 -1.0 0.0))))))
    (:`then_1`
      (if (`self.Right Pressed`)
        (`/Engine/EditorBlueprintResources/StandardMacros.IsValid` _controllerl
          (:`Is Valid`
            (if (== _activeobject_4 null)
              (`/Game/Blueprints/ObjectsBase/iObject.ChangeHue` _activeobject_4 1.0 0.0))))))
    (:`then_2`
      (if (`self.Up Pressed`)
        (`/Engine/EditorBlueprintResources/StandardMacros.IsValid` _controllerr
          (:`Is Valid`
            (if (== _activeobject_2 null)
              (`/Game/Blueprints/ObjectsBase/InteractiveObject.ChangeShape` _activeobject_2 1.0 0.0))))))
    (:`then_3`
      (if (`self.Down Pressed`)
        (`/Engine/EditorBlueprintResources/StandardMacros.IsValid` null
          (:`Is Valid`
            (if (== _activeobject _controllerr)
              (`/Game/Blueprints/ObjectsBase/InteractiveObject.ChangeShape` _activeobject -1.0 0.0))))))))

(event `self.ReceiveBeginPlay`
  ;[1 1 1] On Begin Play
  (`|ExecutionSequence`
    (:`then_0`
      (`HeadMountedDisplayFunctionLibrary.EnableHMD` true)
      (`KismetSystemLibrary.ExecuteConsoleCommand` "fullscreen")
      (`KismetSystemLibrary.ExecuteConsoleCommand` "HMD mirror 2")
      ;;[1 1 1] Oculus
      (`HeadMountedDisplayFunctionLibrary.SetTrackingOrigin` "Floor"))
    (:`then_1`
      (bind _outactors (`GameplayStatics.GetAllActorsOfClass` "/Game/Blueprints/GameSettings/NoiseSpawn.NoiseSpawn_C"))
      (set `self.NoiseSpawn` (`KismetArrayLibrary.Array_Get` _outactors)))
    (:`then_2`
      (`self.StartLevel` 0))))

(event `Key|Left`
  (params (Key :type "Key Structure" :default "AnyKey"))
  ;[1 0 0.7382] REMOVE
  (:`Pressed`
    (set `self.Left Pressed` true))
  (:`Released`
    (set `self.Left Pressed` false)))

(event `Key|Escape`
  (params (Key :type "Key Structure" :default "AnyKey"))
  ;[0.0388 1 0] BUILD
  (:`Pressed`
    (`KismetSystemLibrary.QuitGame` null "Quit")))

(event `Key|Right`
  (params (Key :type "Key Structure" :default "AnyKey"))
  ;[1 0 0.7382] REMOVE
  (:`Pressed`
    (set `self.Right Pressed` true))
  (:`Released`
    (set `self.Right Pressed` false)))

(event `Key|One`
  (params (Key :type "Key Structure" :default "AnyKey"))
  ;[0.0388 1 0] BUILD
  (:`Pressed`
    (`KismetSystemLibrary.ExecuteConsoleCommand` "HMD Mirror mode 4")))

(event `StartLevel`
  (params (Level :type Integer))
  ;[1 1 1] On Begin Play
  (`|ExecutionSequence`
    (:`then_0`
      (bind _outactors (`GameplayStatics.GetAllActorsOfClass` "/Game/Blueprints/ObjectsBase/Instrument.Instrument_C"))
      (bind _output_get (set `self.Instruments` _outactors))
      (for _array_element _output_get
        (`KismetArrayLibrary.Array_Set` (`self.Instruments`) (`/Game/Blueprints/ObjectsBase/Instrument.ID` _array_element) _array_element)))))

(event `Key|Up`
  (params (Key :type "Key Structure" :default "AnyKey"))
  ;[1 0 0.7382] REMOVE
  (:`Pressed`
    (set `self.Up Pressed` true))
  (:`Released`
    (set `self.Up Pressed` false)))

(event `Key|P`
  (params (Key :type "Key Structure" :default "AnyKey"))
  ;[1 1 1] Editor
  (:`Pressed`
    (`KismetSystemLibrary.ExecuteConsoleCommand` "stat FPS")))

(event `Key|R`
  (params (Key :type "Key Structure" :default "AnyKey"))
  ;[1 1 1] Editor
  (:`Pressed`
    (`KismetSystemLibrary.ExecuteConsoleCommand` "RestartLevel")))

(event `Key|Down`
  (params (Key :type "Key Structure" :default "AnyKey"))
  ;[1 0 0.7382] REMOVE
  (:`Pressed`
    (set `self.Down Pressed` true))
  (:`Released`
    (set `self.Down Pressed` false)))

(event `MoveBelt`
  (params (Down :type Boolean))
  (bind (_returnvalue_x _returnvalue_y _returnvalue_z) (`KismetMathLibrary.BreakVector` (`SceneComponent.K2_GetComponentLocation` (`self.Camera`))))
  ;[1 1 1] Move Belt
  (if Down
    (bind (_direction _pos) (`Timeline|InstrumentMovement` :!label _label)
      (:`Update`
        (set `self.BeltZ` (`KismetMathLibrary.Lerp` -50.0 (/ _returnvalue_z -1.5) _pos))
        (`SceneComponent.SetWorldScale3D` (`self.InstrumentCentre`) (`KismetMathLibrary.Conv_DoubleToVector` (`KismetMathLibrary.Lerp` 1.0 4.0 _pos)))))
    (else
      (goto _label :!via `Reverse`))))

(event `InputAxisKey|MouseX`
  (params (AxisValue :type "Float (single-precision)"))
  ;[1 0 0.9084] KEYBOARD CONTROL FOR TESTING
  (if (`self.LMousePressed`)
    _
    (elif (`self.RMousePressed`)
      (`SceneComponent.K2_AddWorldRotation` (`self.Camera`) (`KismetMathLibrary.MakeRotator` 0.0 0.0 AxisValue) false false))))

(event `InputAxisKey|MouseY`
  (params (AxisValue :type "Float (single-precision)"))
  ;[1 0 0.9084] KEYBOARD CONTROL FOR TESTING
  (if (`self.LMousePressed`)
    _
    (elif (`self.RMousePressed`)
      (`SceneComponent.K2_AddLocalRotation` (`self.Camera`) (`KismetMathLibrary.MakeRotator` 0.0 AxisValue) false false))))

(event `self.ReceiveTick`
  (params (DeltaSeconds :type "Float (single-precision)"))
  ;[1 1 1] EventTick
  (`|ExecutionSequence`
    (:`then_0`
      (`self.FollowCameraXY` (`KismetMathLibrary.MakeVector` 0.0 0.0 (`self.BeltZ`)) (`self.InstrumentCentre`))
      (`/Engine/EditorBlueprintResources/StandardMacros.IsValid` (`self.ActiveObject`)
        (:`Is Valid`
          (`self.FollowCameraXY` (`self.ObjectTargetOffset`) (`self.CloseTarget`)))))
    (:`then_1`
      (`self.Keyboad Control`))
    (:`then_2`
      (`self.SumAmplitudes`))))

(event `Key|LeftMouseButton`
  (params (Key :type "Key Structure" :default "AnyKey"))
  ;[1 0 0.9084] KEYBOARD CONTROL FOR TESTING
  (:`Pressed`
    (set `self.LMousePressed` true))
  (:`Released`
    (set `self.LMousePressed` false)))

(event `Key|RightMouseButton`
  (params (Key :type "Key Structure" :default "AnyKey"))
  ;[1 0 0.9084] KEYBOARD CONTROL FOR TESTING
  (:`Pressed`
    (set `self.RMousePressed` true))
  (:`Released`
    (set `self.RMousePressed` false)))

(event `Key|LeftControl`
  (params (Key :type "Key Structure" :default "AnyKey"))
  ;[1 0 0.9084] KEYBOARD CONTROL FOR TESTING
  (:`Pressed`
    (`self.K2_AddActorLocalTransform` (`KismetMathLibrary.MakeTransform` (0.0 0.0 180.0)))))

(event `Key|MotionController_Left_Trigger` :consume false
  (params (Key :type "Key Structure" :default "AnyKey"))
  (bind _controllerl (`self.ControllerL`))
  ;[1 1 1] Button Management
  (:`Pressed`
    (`/Game/Blueprints/GameSettings/Controller/VRController.Trigger Pressed` _controllerl))
  (:`Released`
    (`/Game/Blueprints/GameSettings/Controller/VRController.Trigger Released` _controllerl)))

(event `Key|MotionController_Left_Grip1` :consume false
  (params (Key :type "Key Structure" :default "AnyKey"))
  ;[1 1 1] Button Management
)

(event `Key|U`
  (params (Key :type "Key Structure" :default "AnyKey"))
  ;[1 0 0.9084] KEYBOARD CONTROL FOR TESTING
  (:`Pressed`
    (`SceneComponent.K2_AddLocalOffset` (`self.CapsuleComponent`) (0.0 0.0 10.0) false false)))

(event `Key|MotionController_Left_Thumbstick` :consume false
  (params (Key :type "Key Structure" :default "AnyKey"))
  ;[1 1 1] Button Management
)

(event `Key|MotionController_Right_Trigger` :consume false
  (params (Key :type "Key Structure" :default "AnyKey"))
  (bind _controllerr (`self.ControllerR`))
  ;[1 1 1] Button Management
  (:`Pressed`
    (`/Game/Blueprints/GameSettings/Controller/VRController.Trigger Pressed` _controllerr))
  (:`Released`
    (`/Game/Blueprints/GameSettings/Controller/VRController.Trigger Released` _controllerr)))

(event `Key|MotionController_Right_Grip1` :consume false
  (params (Key :type "Key Structure" :default "AnyKey"))
  ;[1 1 1] Button Management
)

(event `Key|MotionController_Right_Thumbstick` :consume false
  (params (Key :type "Key Structure" :default "AnyKey"))
  ;[1 1 1] Button Management
)

(fn `AddKeep01`
  (params (Base :type "Float (double-precision)") (Add :type "Float (double-precision)"))
  (returns (Out :type "Float (double-precision)"))
  (bind _returnvalue (`KismetMathLibrary.Fraction` (+ Base Add)))
  (if (< _returnvalue 0.0)
    (return (+ _returnvalue 1.0))
    (else
      (return _returnvalue))))

(fn `FollowCameraXY`
  (params (Offset :type "Vector Structure") (Component :type "SceneComponent Object Reference"))
  (bind _returnvalue (`SceneComponent.K2_GetComponentToWorld` Component))
  (bind _returnvalue_2 (`SceneComponent.K2_GetComponentToWorld` (`self.Camera`)))
  (`SceneComponent.K2_SetWorldTransform` Component (`KismetMathLibrary.MakeTransform` (.location _returnvalue_2) (`KismetMathLibrary.MakeRotator` (.roll (.rotation _returnvalue)) (.pitch (.rotation _returnvalue)) (.yaw (.rotation _returnvalue_2))) (.scale _returnvalue)) false false)
  (`SceneComponent.K2_AddLocalOffset` Component Offset false false))

(fn `GetDistance`
  (params (Start :type "Vector Structure") (End :type "Vector Structure"))
  (returns (Distance :type "Float (double-precision)"))
  (return (`KismetMathLibrary.VSize` (- Start End))))

(fn `PingPong01`
  (params (In :type "Float (double-precision)"))
  (returns (Out :type "Float (double-precision)"))
  (bind _returnvalue (`KismetMathLibrary.Fraction` In))
  (if (== (mod (`KismetMathLibrary.FFloor` In) 2) 0)
    (return _returnvalue)
    (else
      (return (- 1.0 _returnvalue)))))

(fn `SumAmplitudes`
  (set `self.AmplitudesSum` 0.0)
  (for _array_element (`self.Amplitudes`)
    (bind _output_get (set `self.AmplitudesSum` (+ (stale _output_get) _array_element)))))

(fn `UserConstructionScript`)