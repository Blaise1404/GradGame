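; VR pawn that lets the player point two gamepad-driven wands at InteractiveObjects and bring one in at a time.
; Thumbstick axes rotate each wand mesh, with X and Y feeding the same combined roll and yaw change.
; Ray cylinder overlaps store each side's target and recolor dynamic ray materials for inactive, active or edit states.
; A trigger with a target brings it in, or puts away the shared active object if one exists.
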(event `/Game/Blueprints/GameSettings/VR_Pawn.ReceiveTick`
  (params (DeltaSeconds :type "Float (single-precision)")))

(event `/Game/Blueprints/GameSettings/VR_Pawn.ReceiveActorBeginOverlap`
  (params (OtherActor :type "Actor Object Reference")))

(event `Key|Gamepad_LeftTrigger` :consume false
  (params (Key :type "Key Structure" :default "AnyKey"))
  (bind _objectl (`self.ObjectL`))
  ;[1 1 1] Bring in
  (:`Pressed`
    (`/Engine/EditorBlueprintResources/StandardMacros.IsValid` _objectl
      (:`Is Valid`
        (`/Engine/EditorBlueprintResources/StandardMacros.IsValid` (`self.ActiveObject`)
          (:`Is Valid`
            (`/Game/Blueprints/InteractiveObject.putAway` (`self.ActiveObject`))
            (set `self.ActiveObject` null))
          (:`Is Not Valid`
            (`/Game/Blueprints/InteractiveObject.bring` _objectl)
            (set `self.ActiveObject` _objectl)))))))

(event `InputAxisKey|Gamepad_RightX` :consume false
  (params (AxisValue :type "Float (single-precision)"))
  (bind _mesh_r (`self.Mesh_R`))
  ;[1 1 1] Wands control
  (`SceneComponent.K2_SetWorldRotation` _mesh_r (`KismetMathLibrary.MakeRotator` (+ (stale `InputAxisKey|Gamepad_RightY` AxisValue) (.roll (`SceneComponent.K2_GetComponentRotation` _mesh_r))) (.pitch (`SceneComponent.K2_GetComponentRotation` _mesh_r)) (+ AxisValue (.yaw (`SceneComponent.K2_GetComponentRotation` _mesh_r)))) false false :!label _label))

(event `InputAxisKey|Gamepad_RightY` :consume false
  (params (AxisValue :type "Float (single-precision)"))
  ;[1 1 1] Wands control
  (goto _label))

(event `Key|Gamepad_RightTrigger`
  (params (Key :type "Key Structure" :default "AnyKey"))
  (bind _objectr (`self.ObjectR`))
  ;[1 1 1] Bring in
  (:`Pressed`
    (`/Engine/EditorBlueprintResources/StandardMacros.IsValid` _objectr
      (:`Is Valid`
        (`/Engine/EditorBlueprintResources/StandardMacros.IsValid` (`self.ActiveObject`)
          (:`Is Valid`
            (`/Game/Blueprints/InteractiveObject.putAway` (`self.ActiveObject`))
            (set `self.ActiveObject` null))
          (:`Is Not Valid`
            (`/Game/Blueprints/InteractiveObject.bring` _objectr)
            (set `self.ActiveObject` _objectr)))))))

(event `InputAxisKey|Gamepad_LeftX` :consume false
  (params (AxisValue :type "Float (single-precision)"))
  (bind _mesh_l (`self.Mesh_L`))
  ;[1 1 1] Wands control
  (`SceneComponent.K2_SetWorldRotation` _mesh_l (`KismetMathLibrary.MakeRotator` (- (.roll (`SceneComponent.K2_GetComponentRotation` _mesh_l)) (stale `InputAxisKey|Gamepad_LeftY` AxisValue)) (.pitch (`SceneComponent.K2_GetComponentRotation` _mesh_l)) (+ AxisValue (.yaw (`SceneComponent.K2_GetComponentRotation` _mesh_l)))) false false :!label _label_2))

(event `InputAxisKey|Gamepad_LeftY` :consume false
  (params (AxisValue :type "Float (single-precision)"))
  ;[1 1 1] Wands control
  (goto _label_2))

(event `/Game/Blueprints/GameSettings/VR_Pawn.ReceiveBeginPlay`
  ;[1 1 1] Enable Input
  (`self.EnableInput` (`GameplayStatics.GetPlayerController` 0)))

(event `self.Cylinder_L.OnComponentBeginOverlap`
  (params (OtherActor :type "Actor Object Reference") (OtherComp :type "PrimitiveComponent Object Reference") (OtherBodyIndex :type Integer) (bFromSweep :type Boolean) (SweepResult :type "HitResult Structure (by ref)"))
  (bind _activeobject (`self.ActiveObject`))
  (bind _matl (`self.MatL`))
  ;[1 1 1] Begin Overlap
  (bind _asinteractive_object (cast `/Game/Blueprints/InteractiveObject` OtherActor))
  (bind _output_get (set `self.ObjectL` _asinteractive_object))
  (`/Engine/EditorBlueprintResources/StandardMacros.IsValid` _activeobject
    (:`Is Valid`
      (if (== _output_get _activeobject)
        (`MaterialInstanceDynamic.SetVectorParameterValue` _matl "Color" (`self.ColorEdit`))))
    (:`Is Not Valid`
      (`MaterialInstanceDynamic.SetVectorParameterValue` _matl "Color" (`self.ColorActive`)))))

(event `self.Cylinder_R.OnComponentBeginOverlap`
  (params (OtherActor :type "Actor Object Reference") (OtherComp :type "PrimitiveComponent Object Reference") (OtherBodyIndex :type Integer) (bFromSweep :type Boolean) (SweepResult :type "HitResult Structure (by ref)"))
  (bind _activeobject (`self.ActiveObject`))
  (bind _matr (`self.MAtR`))
  ;[1 1 1] Begin Overlap
  (bind _asinteractive_object (cast `/Game/Blueprints/InteractiveObject` OtherActor))
  (bind _output_get (set `self.ObjectR` _asinteractive_object))
  (`/Engine/EditorBlueprintResources/StandardMacros.IsValid` _activeobject
    (:`Is Valid`
      (if (== _output_get _activeobject)
        (`MaterialInstanceDynamic.SetVectorParameterValue` _matr "Color" (`self.ColorEdit`))))
    (:`Is Not Valid`
      (`MaterialInstanceDynamic.SetVectorParameterValue` _matr "Color" (`self.ColorActive`)))))

(event `self.Cylinder_R.OnComponentEndOverlap`
  (params (OtherActor :type "Actor Object Reference") (OtherComp :type "PrimitiveComponent Object Reference") (OtherBodyIndex :type Integer))
  ;[1 1 1] End Overlap
  (cast `/Game/Blueprints/InteractiveObject` OtherActor)
  (`MaterialInstanceDynamic.SetVectorParameterValue` (`self.MAtR`) "Color" (`self.ColorInactive`))
  (set `self.ObjectR` null))

(event `self.Cylinder_L.OnComponentEndOverlap`
  (params (OtherActor :type "Actor Object Reference") (OtherComp :type "PrimitiveComponent Object Reference") (OtherBodyIndex :type Integer))
  ;[1 1 1] End Overlap
  (cast `/Game/Blueprints/InteractiveObject` OtherActor)
  (`MaterialInstanceDynamic.SetVectorParameterValue` (`self.MatL`) "Color" (`self.ColorInactive`))
  (set `self.ObjectL` null))

(fn `UserConstructionScript`
  (bind _colorinactive (`self.ColorInactive`))
  (bind _returnvalue (`PrimitiveComponent.CreateDynamicMaterialInstance` (`self.Cylinder_L`) 0 "/Game/Materials/Ray.Ray"))
  (bind _output_get (set `self.MatL` _returnvalue))
  (`MaterialInstanceDynamic.SetVectorParameterValue` _output_get "Color" _colorinactive)
  (bind _returnvalue_2 (`PrimitiveComponent.CreateDynamicMaterialInstance` (`self.Cylinder_R`) 0 "/Game/Materials/Ray.Ray"))
  (bind _output_get_2 (set `self.MAtR` _returnvalue_2))
  (`MaterialInstanceDynamic.SetVectorParameterValue` _output_get_2 "Color" _colorinactive))