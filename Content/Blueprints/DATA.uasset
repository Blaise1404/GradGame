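; DATA is an actor that holds shared references to the VR player and the current world position of the pawn's target.
; On BeginPlay it finds and caches the first VR_PlayerController and VR_Pawn in the level.
; Every Tick it copies the world location of the pawn's Target component into TargetPosition.
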(event `self.ReceiveBeginPlay`
  (bind _outactors (`GameplayStatics.GetAllActorsOfClass` "/Game/Blueprints/GameSettings/VR_PlayerController.VR_PlayerController_C"))
  (set `self.Controller` (`KismetArrayLibrary.Array_Get` _outactors))
  (bind _outactors_2 (`GameplayStatics.GetAllActorsOfClass` "/Game/Blueprints/GameSettings/VR_Pawn.VR_Pawn_C"))
  (set `self.Pawn` (`KismetArrayLibrary.Array_Get` _outactors_2)))

(event `self.ReceiveActorBeginOverlap`
  (params (OtherActor :type "Actor Object Reference")))

(event `self.ReceiveTick`
  (params (DeltaSeconds :type "Float (single-precision)"))
  (set `self.TargetPosition` (`SceneComponent.K2_GetComponentLocation` (`/Game/Blueprints/GameSettings/VR_Pawn.Target` (`self.Pawn`)))))

(fn `UserConstructionScript`)