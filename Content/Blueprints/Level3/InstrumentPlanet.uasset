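; Level 3 instrument planet that reacts to audio amplitude and VR controller contact, building on a parent class.
; BeginPlay randomizes scale and shader parameters, and tints trail and spark dynamic materials with an initial hue.
; Tick runs the visualiser and multiplies the current material speeds by an amplitude-based factor, compounding unless reset elsewhere.
; Controller impacts fire force-scaled sparks, overlaps call Hit, and FollowBelt and GoBack play the object's animation, the latter reversed.
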(event `self.ReceiveTick`
  (params (DeltaSeconds :type "Float (single-precision)"))
  (bind _returnvalue (* (+ (`self.Amplitude`) 1.0) 5.0))
  ;[1 1 1] Tick
  (`parent.ReceiveTick` DeltaSeconds)
  (`self.Visualiser`)
  (`self.RandomizeMaterial` "speedA" _returnvalue)
  (`self.RandomizeMaterial` "speedB" _returnvalue))

(event `self.ReceiveBeginPlay`
  (bind _returnvalue (`KismetMathLibrary.RandomFloatInRange` 0.8 1.2))
  (bind _trail (`self.Trail`))
  (bind _sparks (`self.Sparks`))
  ;[1 1 1] Begin play
  (`parent.ReceiveBeginPlay`)
  (`|ExecutionSequence`
    (:`then_0`
      (`SceneComponent.SetRelativeScale3D` (`self.OrbitTarget`) (* (`SceneComponent.RelativeScale3D` (`self.Object`)) (`KismetMathLibrary.RandomFloatInRange` 0.9 1.12))))
    (:`then_1`
      (bind _returnvalue_2 (`KismetMaterialLibrary.CreateDynamicMaterialInstance` (`PrimitiveComponent.GetMaterial` _trail 0)))
      (bind _output_get (set `self.TrailMat` _returnvalue_2))
      (`PrimitiveComponent.SetMaterial` _trail 0 _output_get)
      (`MaterialInstanceDynamic.SetScalarParameterValue` _output_get "Hue" (`self.InitialHue`)))
    (:`then_2`
      (`self.RandomizeMaterial` "a" _returnvalue)
      (`self.RandomizeMaterial` "b" _returnvalue)
      (`self.RandomizeMaterial` "speedA" _returnvalue)
      (`self.RandomizeMaterial` "speedB" _returnvalue))
    (:`then_3`
      (bind _returnvalue_3 (`PrimitiveComponent.CreateDynamicMaterialInstance` _sparks 0 (`PrimitiveComponent.GetMaterial` _sparks 0)))
      (`PrimitiveComponent.SetMaterial` _sparks 0 _returnvalue_3)
      (`MaterialInstanceDynamic.SetScalarParameterValue` _returnvalue_3 "Hue" (`self.InitialHue`)))))

(event `self.Follow Belt`
  ;[1 1 1] Shape
  (`parent.Follow Belt`)
  (`SkeletalMeshComponent.Play` (`self.Object`) false))

(event `GoBack`
  (bind _object (`self.Object`))
  ;[1 1 1] Shape
  (`SkeletalMeshComponent.SetPlayRate` _object -1.0)
  (`SkeletalMeshComponent.Play` _object false))

(event `self.Object.OnComponentHit`
  (params (HitComponent :type "PrimitiveComponent Object Reference") (OtherActor :type "Actor Object Reference") (OtherComp :type "PrimitiveComponent Object Reference") (NormalImpulse :type "Vector Structure") (Hit :type "HitResult Structure (by ref)"))
  (bind _sparks (`self.Sparks`))
  ;[1 1 1] Overlap
  (cast `/Game/Blueprints/GameSettings/Controller/VRController` OtherActor)
  (`SceneComponent.K2_SetWorldLocation` _sparks (`.Location` (`GameplayStatics.BreakHitResult` Hit)) false false)
  (`SceneComponent.SetWorldScale3D` _sparks (`KismetMathLibrary.Conv_DoubleToVector` (`KismetMathLibrary.FClamp` (`KismetMathLibrary.VSize` NormalImpulse) 0.1 0.2)))
  (`ActorComponent.SetActive` _sparks true false))

(event `self.Collider.OnComponentBeginOverlap`
  (params (OverlappedComponent :type "PrimitiveComponent Object Reference") (OtherActor :type "Actor Object Reference") (OtherComp :type "PrimitiveComponent Object Reference") (OtherBodyIndex :type Integer) (bFromSweep :type Boolean) (SweepResult :type "HitResult Structure (by ref)"))
  ;[1 1 1] Overlap
  (bind _asvrcontroller (cast `/Game/Blueprints/GameSettings/Controller/VRController` OtherActor))
  (`self.Hit` (`/Game/Blueprints/GameSettings/Controller/VRController.Controller Mesh` _asvrcontroller)))

(fn `RandomizeMaterial`
  (params (Name :type Name) (Multiplier :type "Float (double-precision)"))
  (bind _item (`KismetArrayLibrary.Array_Get` (`self.MaterialsDynamic`)))
  (bind _returnvalue (`MaterialInstanceDynamic.K2_GetScalarParameterValue` _item Name))
  (`MaterialInstanceDynamic.SetScalarParameterValue` _item Name (* _returnvalue Multiplier)))

(fn `UserConstructionScript`
  (`parent.UserConstructionScript`))