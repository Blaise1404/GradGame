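; Level 3 environment actor that drives its cone materials from the VR character's summed amplitude value.
; The construction script builds a materials set from the ConeVertical and ConeHorizontal components.
; BeginPlay caches the first VR_Character found in the world, and every Tick passes its AmplitudesSum and those materials to ApplyVis to update the visualization.
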(event `self.ReceiveBeginPlay`
  (bind _outactors (`GameplayStatics.GetAllActorsOfClass` "/Game/Blueprints/GameSettings/VR_Character.VR_Character_C"))
  (set `self.Character` (`KismetArrayLibrary.Array_Get` _outactors)))

(event `self.ReceiveTick`
  (params (DeltaSeconds :type "Float (single-precision)"))
  (`/Game/Blueprints/GeneralFunctions/DynamicMaterials.ApplyVis` (`self.Materials`) (`/Game/Blueprints/GameSettings/VR_Character.AmplitudesSum` (`self.Character`))))

(fn `UserConstructionScript`
  (bind _materials (`/Game/Blueprints/GeneralFunctions/DynamicMaterials.SetMaterials` (`|MakeArray` (`self.cone_vertical`) (`self.cone_horizontal`) :!type "MeshComponent Object Reference")))
  (set `self.Materials` _materials))