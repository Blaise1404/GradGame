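; CrystalStar2 is a Level3_2 crystal star Blueprint that extends a parent class's shape-change behavior with a material UV effect.
; Its ChangeShape override calls the parent, then sets the CrystalsUV timeline's time to the Shape value instead of playing it.
; The timeline update writes its UV track to the "UV" scalar parameter on every dynamic material except the first.
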(event `self.ChangeShape`
  (params (Value :type "Float (single-precision)") (Add :type "Float (single-precision)"))
  (`parent.ChangeShape` Value Add)
  (bind (_direction _uv) (`Timeline|CrystalsUV` :`NewTime` (`self.Shape`) :!via `SetNewTime`)
    (:`Update`
      (for (_array_element _array_index) (`self.MaterialsDynamic`)
        (if (> _array_index 0)
          (`MaterialInstanceDynamic.SetScalarParameterValue` _array_element "UV" _uv))))))

(fn `UserConstructionScript`
  (`parent.UserConstructionScript`))