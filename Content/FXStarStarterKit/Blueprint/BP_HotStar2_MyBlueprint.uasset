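; BP_HotStar2_MyBlueprint is a star actor that links player input to FMOD audio and star colors.
; Vertical input cycles Filter, driving the FMOD parameter and the hue of the hot and warm surface colors, with warm offset slightly.
; Horizontal input cycles Pitch, driving its FMOD parameter and the atmosphere hue.
; Both values are applied on BeginPlay and each input, writing colors to a dynamic material while preserving saturation and brightness.
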(event `self.ReceiveBeginPlay`
  (bind _star_dm_b (`self.Star_DM_B`))
  (`|ExecutionSequence`
    (:`then_0`
      (`FMODAudioComponent.SetParameter` (`self.FMODAudio`) "Filter" (stale _output_get) :!label _label)
      (bind (_h _s _v _a) (`KismetMathLibrary.RGBToHSV` (stale _output_get)))
      (bind _output_get (set `self.SurfaceKelvin_Hot` (`KismetMathLibrary.HSVToRGB` (* (stale _output_get) 360.0) _s _v _a)))
      (bind (_h_2 _s_2 _v_2 _a_2) (`KismetMathLibrary.RGBToHSV` (stale _output_get_2)))
      (bind _output_get_2 (set `self.SurfaceKelvin_Warm` (`KismetMathLibrary.HSVToRGB` (+ (* (stale _output_get) 360.0) 20.0) _s_2 _v_2 _a_2)))
      (`MaterialInstanceDynamic.SetVectorParameterValue` _star_dm_b "KH_SurfaceHot" _output_get)
      (`MaterialInstanceDynamic.SetVectorParameterValue` _star_dm_b "KH_SurfaceWarm" _output_get_2))
    (:`then_1`
      (`FMODAudioComponent.SetParameter` (`self.FMODAudio`) "Pitch" (stale _output_get) :!label _label_2)
      (bind (_h_3 _s_3 _v_3 _a_3) (`KismetMathLibrary.RGBToHSV` (stale _output_get_3)))
      (bind _output_get_3 (set `self.Atmosphere_Kelvin` (`KismetMathLibrary.HSVToRGB` (* (stale _output_get) 360.0) _s_3 _v_3 _a_3)))
      (`MaterialInstanceDynamic.SetVectorParameterValue` (`self.Star_DM_B`) "KH_AtmoHot" _output_get_3))))

(event `self.ReceiveActorBeginOverlap`
  (params (OtherActor :type "Actor Object Reference")))

(event `self.ReceiveTick`
  (params (DeltaSeconds :type "Float (single-precision)")))

(event `Player Vertical Input`
  (params (Value :type "Float (double-precision)"))
  (bind _output_get (set `self.Filter` (mod (+ (stale _output_get) (/ Value 360.0)) 1.0)))
  (goto _label))

(event `Player Horizontal Input`
  (params (Value :type "Float (double-precision)"))
  (bind _output_get (set `self.Pitch` (mod (+ (stale _output_get) (/ Value 360.0)) 1.0)))
  (goto _label_2))

(fn `UserConstructionScript`
  (`parent.UserConstructionScript`))